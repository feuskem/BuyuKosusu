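; BP_Puddle is a puddle actor that shows an ice mesh when a BP_Ice actor overlaps its box.
; On overlap it unhides the ice and runs timelines that animate the ice's Z scale and the puddle's XY scale.
; Five seconds after overlap ends, separate timelines rescale both meshes and hide the ice when finished.
; The ScaledAlready flag, set during timeline updates, gates the two transitions.
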(event OnComponentBeginOverlap(Box)
  (params (OverlappedComponent :type Primitive%20Component%20Object%20Reference) (OtherActor :type Actor%20Object%20Reference) (OtherComp :type Primitive%20Component%20Object%20Reference) (OtherBodyIndex :type Integer) (bFromSweep :type Boolean) (SweepResult :type Hit%20Result%20Structure%20%28by%20ref%29))
  (Utilities|Casting|CastToBP_Ice OtherActor)
  (if (not (Variables|Default|GetScaledAlready))
    (Development|SetHiddeninGame (Variables|Default|Getice) false false)
    (Utilities|FlowControl|Sequence
      (:then_0
        (bind _newtrack_0 (Timeline|ScaleZ PlayFromStart)
          (:Update
            (Transformation|SetWorldScale3D (Variables|Default|Getice) (Math|Vector|MakeVector 2.0 2.0 _newtrack_0))
            (Variables|Default|SetScaledAlready true))))
      (:then_1
        (bind _newtrack_0_2 (Timeline|Timeline PlayFromStart)
          (:Update
            (Transformation|SetWorldScale3D (Variables|Default|Getpuddle) (Math|Vector|MakeVector _newtrack_0_2 _newtrack_0_2 0.02))))))))

(event OnComponentEndOverlap(Box)
  (params (OverlappedComponent :type Primitive%20Component%20Object%20Reference) (OtherActor :type Actor%20Object%20Reference) (OtherComp :type Primitive%20Component%20Object%20Reference) (OtherBodyIndex :type Integer))
  (Utilities|Casting|CastToBP_Ice OtherActor)
  (Utilities|FlowControl|Delay 5.0)
  (if (Variables|Default|GetScaledAlready)
    (Utilities|FlowControl|Sequence
      (:then_0
        (bind _newtrack_0 (Timeline|Timeline_0 PlayFromStart)
          (:Update
            (Transformation|SetWorldScale3D (Variables|Default|Getpuddle) (Math|Vector|MakeVector _newtrack_0 _newtrack_0 0.02))
            (Variables|Default|SetScaledAlready false))))
      (:then_1
        (bind _newtrack_0_2 (Timeline|Timeline_1 PlayFromStart)
          (:Update
            (Transformation|SetWorldScale3D (Variables|Default|Getice) (Math|Vector|MakeVector 2.0 2.0 _newtrack_0_2)))
          (:Finished
            (Development|SetHiddeninGame (Variables|Default|Getice) true false)))))))

(event EventBeginPlay)

(event Collision|EventActorBeginOverlap
  (params (OtherActor :type Actor%20Object%20Reference)))

(event EventTick
  (params (DeltaSeconds :type Float%20%28single-precision%29)))

(fn ConstructionScript)