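; BP_Collectibles is a collectible artifact that the first-person character picks up by touching its sphere.
; On overlap it increments the artifact count on BP_ObjectiveManager, found at BeginPlay, plays a collect sound and destroys itself.
; A Mark event briefly reveals the otherwise hidden Light component, with a timeline driving the opacity of its dynamic material before hiding it again.
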(event OnComponentBeginOverlap(Sphere)
  (params (OverlappedComponent :type Primitive%20Component%20Object%20Reference) (OtherActor :type Actor%20Object%20Reference) (OtherComp :type Primitive%20Component%20Object%20Reference) (OtherBodyIndex :type Integer) (bFromSweep :type Boolean) (SweepResult :type Hit%20Result%20Structure%20%28by%20ref%29))
  (Utilities|Casting|CastToBP_FirstPersonCharacter OtherActor)
  (bind _result (Math|Integer|IncrementInt (Variables|/Game/Blueprints/BP_ObjectiveManager.BP_ObjectiveManager_C|GetArtifactCurrentAmount (stale EventBeginPlay _returnvalue)))
    (:%20%20
      (Variables|/Game/Blueprints/BP_ObjectiveManager.BP_ObjectiveManager_C|SetArtifactCurrentAmount (stale EventBeginPlay _returnvalue) _result)
      (Audio|PlaySound2D "/Game/SFX/Collect.Collect" 1.0 1.0 0.0 0 0)
      (Actor|DestroyActor))))

(event EventBeginPlay
  (bind _returnvalue (Actor|GetActorOfClass "/Game/Blueprints/BP_ObjectiveManager.BP_ObjectiveManager_C"))
  (Rendering|SetVisibility (Variables|Default|GetLight) false false)
  (bind _returnvalue_2 (Rendering|Material|CreateDynamicMaterialInstance (Variables|Default|GetLight) 0 "/Game/Materials/M_Bun.M_Bun" "None" :!class /Script/Engine.PrimitiveComponent))
  (Variables|Default|SetMaterialLight _returnvalue_2))

(event Collision|EventActorBeginOverlap
  (params (OtherActor :type Actor%20Object%20Reference)))

(event EventTick
  (params (DeltaSeconds :type Float%20%28single-precision%29)))

(event EventMark
  (Rendering|SetVisibility (Variables|Default|GetLight) true false)
  (bind _newtrack_0 (Timeline|Opacity PlayFromStart)
    (:Update
      (Rendering|Material|SetScalarParameterValue (Variables|Default|GetMaterialLight) "OpacityValue" _newtrack_0 :!class /Script/Engine.MaterialInstanceDynamic))
    (:Finished
      (Rendering|SetVisibility (Variables|Default|GetLight) false false))))

(fn ConstructionScript)