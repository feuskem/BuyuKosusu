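; Enemy turret that tracks the first-person player, fires projectiles, and is destroyed on overlap with a deflect projectile.
; Pawn sensing turns the body's yaw toward the player and aims the gun with interpolated, pitch-clamped rotation.
; Each sighting also restarts a retriggerable delay, which spawns a projectile at the Spawn transform upon expiry.
; A sphere overlap snaps the whole actor to face the player.
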(event OnSeePawn(PawnSensing)
  (params (Pawn :type Pawn%20Object%20Reference))
  (bind _asbp_first_person_character (Utilities|Casting|CastToBP_FirstPersonCharacter Pawn))
  (Utilities|FlowControl|Sequence
    (:then_0
      (Transformation|SetWorldRotation (Variables|Default|GetGun) (Math|Rotator|MakeRotator 0.0 (Math|Float|Clamp(Float) (.pitch (Math|Interpolation|RInterpTo (Transformation|GetActorRotation) (Math|Rotator|FindLookatRotation (Transformation|GetActorLocation) (Transformation|GetActorLocation _asbp_first_person_character)) (Utilities|Time|GetWorldDeltaSeconds) (* 2e+01 5.0))) -2e+01 2e+01) (.yaw (Math|Interpolation|RInterpTo (Transformation|GetActorRotation) (Math|Rotator|FindLookatRotation (Transformation|GetActorLocation) (Transformation|GetActorLocation _asbp_first_person_character)) (Utilities|Time|GetWorldDeltaSeconds) (* 2e+01 5.0)))) false false)
      (Transformation|SetActorRotation (Math|Rotator|MakeRotator 0.0 0.0 (.yaw (Math|Interpolation|RInterpTo (Transformation|GetActorRotation) (Math|Rotator|FindLookatRotation (Transformation|GetActorLocation) (Transformation|GetActorLocation _asbp_first_person_character)) (Utilities|Time|GetWorldDeltaSeconds) (* 2e+01 5.0))))))
    (:then_1
      (Utilities|FlowControl|RetriggerableDelay 0.5)
      (Game|SpawnActorfromClass "/Game/Blueprints/BP_Projectile_Child.BP_Projectile_Child_C" (Transformation|GetWorldTransform (Variables|Default|GetSpawn)) "Undefined" "MultiplyWithRoot" 0 0))))

(event OnComponentBeginOverlap(Sphere)
  (params (OverlappedComponent :type Primitive%20Component%20Object%20Reference) (OtherActor :type Actor%20Object%20Reference) (OtherComp :type Primitive%20Component%20Object%20Reference) (OtherBodyIndex :type Integer) (bFromSweep :type Boolean) (SweepResult :type Hit%20Result%20Structure%20%28by%20ref%29))
  (bind _asbp_first_person_character (Utilities|Casting|CastToBP_FirstPersonCharacter OtherActor))
  (Transformation|SetActorRotation (Math|Rotator|MakeRotator 0.0 (.pitch (Math|Rotator|FindLookatRotation (Transformation|GetActorLocation) (Transformation|GetActorLocation _asbp_first_person_character))) (.yaw (Math|Rotator|FindLookatRotation (Transformation|GetActorLocation) (Transformation|GetActorLocation _asbp_first_person_character))))))

(event EventBeginPlay)

(event Collision|EventActorBeginOverlap
  (params (OtherActor :type Actor%20Object%20Reference))
  (Utilities|Casting|CastToBP_Projectile_Deflect OtherActor)
  (Actor|DestroyActor))

(event EventTick
  (params (DeltaSeconds :type Float%20%28single-precision%29)))

(fn ConstructionScript)