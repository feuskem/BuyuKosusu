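; Objective manager actor that sets and tracks per-level enemy-kill and artifact-collection goals across Level 1, 2 and 3.
; On BeginPlay it picks targets and objective-type flags from the level name, provided the player pawn is BP_FirstPersonCharacter.
; A 0.1-second timer polls Update, which compares current counts to targets and sets individual and combined completion flags.
; Counts are not incremented here, and the OnObjectiveUpdated dispatcher call is unconnected.
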(event Custom|Update
  (Utilities|Time|SetTimerbyEvent (delegate Custom|Update) 0.1 true)
  (switch string (stale EventBeginPlay _returnvalue)
    (:Level1
      _)
    (:Level2
      _)
    (:Level3
      _))
  (Utilities|FlowControl|Sequence
    (:then_0
      (if (== (Variables|Default|GetEnemyObjective) (Variables|Default|GetEnemyCurrentAmount))
        (Variables|Default|SetEnemyObjectiveCompleted true)
        (else
          (Variables|Default|SetEnemyObjectiveCompleted false))))
    (:then_1
      (if (== (Variables|Default|GetArtifactObjective) (Variables|Default|GetArtifactCurrentAmount))
        (Variables|Default|SetArtifactObjectiveCompleted true)
        (else
          (Variables|Default|SetArtifactObjectiveCompleted false))))
    (:then_2
      (if (and (Variables|Default|GetEnemyObjectiveCompleted) (Variables|Default|GetArtifactObjectiveCompleted))
        (Variables|Default|SetBothObjectivesCompleted true)
        (else
          (Variables|Default|SetBothObjectivesCompleted false))))))

(event EventBeginPlay
  (CallFunction|Update)
  (Utilities|Casting|CastToBP_FirstPersonCharacter (Game|Player|GetPlayerPawn 0))
  (bind _returnvalue (Game|GetCurrentLevelName true))
  (switch string _returnvalue
    (:Level1
      (Variables|Default|SetBothObjectivesCompleted false)
      (Variables|Default|SetEnemyCurrentAmount 0)
      (Variables|Default|SetEnemyObjective 6)
      (Variables|Default|SetArtifactObjective 0)
      (Variables|Default|SetArtifactCurrentAmount 0)
      (Variables|Default|SetIsKillingEnemiesObjective true))
    (:Level2
      (Variables|Default|SetIsColletingArtifactsObjective true)
      (Variables|Default|SetIsKillingEnemiesObjective true)
      (Variables|Default|SetEnemyObjective 12)
      (Variables|Default|SetEnemyCurrentAmount 0)
      (Variables|Default|SetArtifactObjective 2))
    (:Level3
      (Variables|Default|SetIsColletingArtifactsObjective true)
      (Variables|Default|SetIsKillingEnemiesObjective true)
      (Variables|Default|SetEnemyObjective 17)
      (Variables|Default|SetArtifactObjective 1))))

(event Collision|EventActorBeginOverlap
  (params (OtherActor :type Actor%20Object%20Reference)))

(event EventTick
  (params (DeltaSeconds :type Float%20%28single-precision%29)))

(fn ConstructionScript)