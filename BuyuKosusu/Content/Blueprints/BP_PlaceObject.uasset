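; BP_PlaceObject is a placement spot that snaps a BP_GrabActor into position when it enters the Box trigger.
; On overlap, it disables physics on the actor's Cube and teleports the actor to the StaticMesh's world location without changing its rotation.
; An Inside flag blocks further snaps until any end-overlap event on the Box clears it, regardless of which actor left.
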(event OnComponentBeginOverlap(Box)
  (params (OverlappedComponent :type Primitive%20Component%20Object%20Reference) (OtherActor :type Actor%20Object%20Reference) (OtherComp :type Primitive%20Component%20Object%20Reference) (OtherBodyIndex :type Integer) (bFromSweep :type Boolean) (SweepResult :type Hit%20Result%20Structure%20%28by%20ref%29))
  (if (not (Variables|Default|GetInside))
    (bind _asbp_grab_actor (Utilities|Casting|CastToBP_GrabActor OtherActor))
    (Physics|SetSimulatePhysics (Variables|/Game/Blueprints/BP_GrabActor.BP_GrabActor_C|GetCube _asbp_grab_actor) false)
    (Transformation|SetActorLocation _asbp_grab_actor (Transformation|GetWorldLocation (Variables|Default|GetStaticMesh)) false false)
    (Variables|Default|SetInside true)))

(event OnComponentEndOverlap(Box)
  (params (OverlappedComponent :type Primitive%20Component%20Object%20Reference) (OtherActor :type Actor%20Object%20Reference) (OtherComp :type Primitive%20Component%20Object%20Reference) (OtherBodyIndex :type Integer))
  (Variables|Default|SetInside false))

(event EventBeginPlay)

(event Collision|EventActorBeginOverlap
  (params (OtherActor :type Actor%20Object%20Reference)))

(event EventTick
  (params (DeltaSeconds :type Float%20%28single-precision%29)))

(fn ConstructionScript)