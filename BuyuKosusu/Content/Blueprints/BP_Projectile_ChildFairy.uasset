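; BP_Projectile_ChildFairy is a child projectile that damages the first-person player on overlap.
; Its sphere ignores enemy turrets, destroys the projectile when it hits the player's parry capsule child, and applies damage when it hits the body capsule.
; A timeline started on BeginPlay adds to its scale each update.
; Every tick a downward line trace moves a plane to the ground height beneath it, like a landing marker.
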(event OnComponentBeginOverlap(Sphere)
  (params (OverlappedComponent :type Primitive%20Component%20Object%20Reference) (OtherActor :type Actor%20Object%20Reference) (OtherComp :type Primitive%20Component%20Object%20Reference) (OtherBodyIndex :type Integer) (bFromSweep :type Boolean) (SweepResult :type Hit%20Result%20Structure%20%28by%20ref%29))
  (if (not (Class|GameplayStatics|ObjectIsA OtherActor "/Game/Blueprints/Enemies/BP_EnemyTurret.BP_EnemyTurret_C"))
    (if (== OtherComp (Components|GetChildComponent (Variables|/Game/FirstPerson/Blueprints/BP_FirstPersonCharacter.BP_FirstPersonCharacter_C|GetParryCapsule (stale EventBeginPlay _asbp_first_person_character)) 0))
      (Actor|DestroyActor)
      (elif (== OtherComp (Variables|/Script/Engine.Character|GetCapsuleComponent (stale EventBeginPlay _asbp_first_person_character)))
        (Game|Damage|ApplyDamage (stale EventBeginPlay _asbp_first_person_character) 3e+01 0 0)))))

(event EventBeginPlay
  (|CallParentFunction)
  (Variables|Default|SetAAA (Transformation|GetActorTransform))
  (bind _asbp_first_person_character (Utilities|Casting|CastToBP_FirstPersonCharacter (Game|Player|GetPlayerPawn 0)))
  (bind _newtrack_0 (Timeline|Scale PlayFromStart)
    (:Update
      (Transformation|SetActorScale3D (+ (Transformation|GetActorScale3D) (Math|Conversions|ToVector(Float) _newtrack_0))))))

(event Collision|EventActorBeginOverlap
  (params (OtherActor :type Actor%20Object%20Reference)))

(event EventTick
  (params (DeltaSeconds :type Float%20%28single-precision%29))
  (bind _returnvalue (Transformation|GetActorLocation))
  (bind _returnvalue_2 (Transformation|GetActorLocation))
  (bind (_outhit _returnvalue_3) (Collision|LineTraceByChannel (Transformation|GetActorLocation) (Math|Vector|MakeVector (.x _returnvalue) (.y _returnvalue) (- (.z _returnvalue) 1e+03)) "TraceTypeQuery3" true 0 "None"))
  (if _returnvalue_3
    (Transformation|SetWorldLocation (Variables|Default|GetPlane) (Math|Vector|MakeVector (.x _returnvalue_2) (.y _returnvalue_2) (.z (.ImpactPoint (Collision|BreakHitResult _outhit)))) false false)))

(fn ConstructionScript
  (|CallParentFunction))