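; Enemy-style water projectile that deals fixed damage to the first-person player and flags an ink hit on the HUD.
; BeginPlay caches the player pawn as BP_FirstPersonCharacter.
; Sphere overlap with that character's capsule applies damage, sets the HUD's InkHit flag and destroys the projectile.
; Both collision spheres also destroy it on overlapping components of a custom collision channel (GameTraceChannel7).
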(event OnComponentBeginOverlap(Sphere)
  (params (OverlappedComponent :type Primitive%20Component%20Object%20Reference) (OtherActor :type Actor%20Object%20Reference) (OtherComp :type Primitive%20Component%20Object%20Reference) (OtherBodyIndex :type Integer) (bFromSweep :type Boolean) (SweepResult :type Hit%20Result%20Structure%20%28by%20ref%29))
  (Utilities|FlowControl|Sequence
    (:then_0
      (if (== OtherComp (Variables|/Script/Engine.Character|GetCapsuleComponent (stale EventBeginPlay _asbp_first_person_character)))
        (Game|Damage|ApplyDamage (Variables|Default|GetAs%20BP%20First%20Person%20Character) 2e+01 0 0)
        (Variables|/Game/W_HUD.W_HUD_C|SetInkHit (Variables|/Game/FirstPerson/Blueprints/BP_FirstPersonCharacter.BP_FirstPersonCharacter_C|GetHudRef (stale EventBeginPlay _asbp_first_person_character)) true)
        (Actor|DestroyActor)))
    (:then_1
      (if (Utilities|Enum|Equal(Enum) (Collision|GetCollisionObjectType (stale OnComponentBeginOverlap(Sphere1_0) OtherComp)) "ECC_GameTraceChannel7")
        (Actor|DestroyActor)))))

(event OnComponentBeginOverlap(Sphere1_0)
  (params (OverlappedComponent :type Primitive%20Component%20Object%20Reference) (OtherActor :type Actor%20Object%20Reference) (OtherComp :type Primitive%20Component%20Object%20Reference) (OtherBodyIndex :type Integer) (bFromSweep :type Boolean) (SweepResult :type Hit%20Result%20Structure%20%28by%20ref%29))
  (if (Utilities|Enum|Equal(Enum) (Collision|GetCollisionObjectType OtherComp) "ECC_GameTraceChannel7")
    (Actor|DestroyActor)))

(event EventBeginPlay
  (|CallParentFunction)
  (bind _asbp_first_person_character (Utilities|Casting|CastToBP_FirstPersonCharacter (Game|Player|GetPlayerPawn 0)))
  (Variables|Default|SetAs%20BP%20First%20Person%20Character _asbp_first_person_character))

(event Collision|EventActorBeginOverlap
  (params (OtherActor :type Actor%20Object%20Reference))
  (|CallParentFunction OtherActor) ; This node is disabled and will not be called.\nDrag off pins to build functionality.
)

(event EventTick
  (params (DeltaSeconds :type Float%20%28single-precision%29))
  (|CallParentFunction DeltaSeconds) ; This node is disabled and will not be called.\nDrag off pins to build functionality.
)

(fn ConstructionScript
  (|CallParentFunction))