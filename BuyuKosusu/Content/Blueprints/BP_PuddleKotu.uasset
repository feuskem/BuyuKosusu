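; BP_PuddleKotu is a short-lived puddle actor whose Ice component animates its height, then removes itself.
; On BeginPlay, the ScaleZ timeline drives the Ice Z scale and its updates feed a three-second Delay.
; After the delay, the ScaledAlready flag lets Timeline_1 start once to drive Z again, then hide Ice and destroy the actor on finish.
; The Box overlap events do nothing.
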(event OnComponentBeginOverlap(Box)
  (params (OverlappedComponent :type Primitive%20Component%20Object%20Reference) (OtherActor :type Actor%20Object%20Reference) (OtherComp :type Primitive%20Component%20Object%20Reference) (OtherBodyIndex :type Integer) (bFromSweep :type Boolean) (SweepResult :type Hit%20Result%20Structure%20%28by%20ref%29)))

(event OnComponentEndOverlap(Box)
  (params (OverlappedComponent :type Primitive%20Component%20Object%20Reference) (OtherActor :type Actor%20Object%20Reference) (OtherComp :type Primitive%20Component%20Object%20Reference) (OtherBodyIndex :type Integer)))

(event Collision|EventActorBeginOverlap
  (params (OtherActor :type Actor%20Object%20Reference)))

(event EventTick
  (params (DeltaSeconds :type Float%20%28single-precision%29)))

(event EventBeginPlay
  (if (not (Variables|Default|GetScaledAlready))
    (Variables|Default|SetScaledAlready true)
    (Utilities|FlowControl|Sequence
      (:then_0
        (bind _newtrack_0 (Timeline|ScaleZ PlayFromStart)
          (:Update
            (Transformation|SetWorldScale3D (Variables|Default|Getice) (Math|Vector|MakeVector 1.0 1.0 _newtrack_0))
            (Utilities|FlowControl|Delay 3.0)
            (if (Variables|Default|GetScaledAlready)
              (Variables|Default|SetScaledAlready false)
              (Utilities|FlowControl|Sequence
                (:then_1
                  (bind _newtrack_0_2 (Timeline|Timeline_1 PlayFromStart)
                    (:Update
                      (Transformation|SetWorldScale3D (Variables|Default|Getice) (Math|Vector|MakeVector 1.0 1.0 _newtrack_0_2)))
                    (:Finished
                      (Development|SetHiddeninGame (Variables|Default|Getice) true false)
                      (Actor|DestroyActor))))))))))))

(fn ConstructionScript)