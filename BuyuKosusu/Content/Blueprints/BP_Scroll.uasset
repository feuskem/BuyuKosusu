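; BP_Scroll is a pickup that grants the first-person player one scroll of its configured Scroll type.
; On BeginPlay it picks the mesh material for that type, with Ice also resetting the Niagara asset.
; Two timelines chain endlessly to animate its height by adding offsets to its current Z.
; Box overlap by the player increments that type in the ScrollAmount map, plays HUD pickup animations and destroys the actor.
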(event OnComponentBeginOverlap(Box)
  (params (OverlappedComponent :type Primitive%20Component%20Object%20Reference) (OtherActor :type Actor%20Object%20Reference) (OtherComp :type Primitive%20Component%20Object%20Reference) (OtherBodyIndex :type Integer) (bFromSweep :type Boolean) (SweepResult :type Hit%20Result%20Structure%20%28by%20ref%29))
  (bind _scroll (Variables|Default|GetScroll))
  (bind _asbp_first_person_character (Utilities|Casting|CastToBP_FirstPersonCharacter OtherActor))
  (if true
    (Utilities|Map|Add (Variables|/Game/FirstPerson/Blueprints/BP_FirstPersonCharacter.BP_FirstPersonCharacter_C|GetScrollAmount _asbp_first_person_character) _scroll (+ (.Value (Utilities|Map|Find (Variables|/Game/FirstPerson/Blueprints/BP_FirstPersonCharacter.BP_FirstPersonCharacter_C|GetScrollAmount _asbp_first_person_character) _scroll)) 1))
    (Variables|/Game/W_HUD.W_HUD_C|SetTakenScroll (Variables|/Game/FirstPerson/Blueprints/BP_FirstPersonCharacter.BP_FirstPersonCharacter_C|GetHudRef _asbp_first_person_character) _scroll)
    (UserInterface|Animation|PlayAnimation (Variables|/Game/FirstPerson/Blueprints/BP_FirstPersonCharacter.BP_FirstPersonCharacter_C|GetHudRef _asbp_first_person_character) (Variables|/Game/W_HUD.W_HUD_C|GetScrollTaken (Variables|/Game/FirstPerson/Blueprints/BP_FirstPersonCharacter.BP_FirstPersonCharacter_C|GetHudRef _asbp_first_person_character)) 0.0 1 "Forward" 1.0 false)
    (UserInterface|Animation|PlayAnimation (Variables|/Game/FirstPerson/Blueprints/BP_FirstPersonCharacter.BP_FirstPersonCharacter_C|GetHudRef _asbp_first_person_character) (Variables|/Game/W_HUD.W_HUD_C|GetScrollTkaenSymbol (Variables|/Game/FirstPerson/Blueprints/BP_FirstPersonCharacter.BP_FirstPersonCharacter_C|GetHudRef _asbp_first_person_character)) 0.0 1 "Forward" 1.0 false)
    (Actor|DestroyActor)))

(event Custom|bum
  (bind _returnvalue (Transformation|GetActorLocation))
  (bind _newtrack_0 (Timeline|Timeline PlayFromStart)
    (:Update
      (Transformation|SetActorLocation (Math|Vector|MakeVector (.x _returnvalue) (.y _returnvalue) (+ (.z _returnvalue) _newtrack_0)) false false))
    (:Finished
      (bind _newtrack_0_2 (Timeline|Timeline_0 PlayFromStart)
        (:Update
          (Transformation|SetActorLocation (Math|Vector|MakeVector (.x _returnvalue) (.y _returnvalue) (+ (.z _returnvalue) _newtrack_0_2)) false false))
        (:Finished
          (Timeline|Timeline PlayFromStart))))))

(event EventBeginPlay
  (bind _staticmesh (Variables|Default|GetStaticMesh))
  (CallFunction|Bum)
  (Utilities|Casting|CastToBP_FirstPersonCharacter (Game|Player|GetPlayerPawn 0))
  (switch Utilities|FlowControl|Switch|SwitchonE_ScrollType (Variables|Default|GetScroll)
    (:NewEnumerator0
      (Rendering|Material|SetMaterial _staticmesh 0 "/Game/Materials/Scrollmaterials/scrollsnow.scrollsnow")
      (Class|NiagaraComponent|SetAsset (Variables|Default|GetNiagara) 0 true))
    (:NewEnumerator1
      (Rendering|Material|SetMaterial _staticmesh 0 "/Game/Materials/Scrollmaterials/scrollmagnet.scrollmagnet"))
    (:NewEnumerator3
      (Rendering|Material|SetMaterial _staticmesh 0 "/Game/Materials/Scrollmaterials/scrollteleport.scrollteleport"))
    (:NewEnumerator4
      (Rendering|Material|SetMaterial _staticmesh 0 "/Game/Materials/Scrollmaterials/scrolldash.scrolldash"))
    (:NewEnumerator5
      (Rendering|Material|SetMaterial _staticmesh 0 "/Game/Materials/Scrollmaterials/scrolldagger.scrolldagger"))
    (:NewEnumerator6
      (Rendering|Material|SetMaterial _staticmesh 0 "/Game/Materials/Scrollmaterials/scrollcheckpoint.scrollcheckpoint"))
    (:NewEnumerator7
      (Rendering|Material|SetMaterial _staticmesh 0 "/Game/Materials/Scrollmaterials/scrollshield.scrollshield"))))

(event Collision|EventActorBeginOverlap
  (params (OtherActor :type Actor%20Object%20Reference)))

(event EventTick
  (params (DeltaSeconds :type Float%20%28single-precision%29)))

(fn ConstructionScript)