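; BP_Trap is a one-shot trap that briefly immobilizes the first-person character.
; Its sphere overlap disarms it, swaps and rescales the mesh, and calls Slow, which nearly zeroes walk speed, disables jumping and sets character flag A.
; Slow re-applies this on a looping timer until a delay ends, when the timer clears and hardcoded movement values are restored.
; A BP_Fireball overlap also disarms the trap and changes its mesh.
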(event OnComponentBeginOverlap(Sphere)
  (params (OverlappedComponent :type Primitive%20Component%20Object%20Reference) (OtherActor :type Actor%20Object%20Reference) (OtherComp :type Primitive%20Component%20Object%20Reference) (OtherBodyIndex :type Integer) (bFromSweep :type Boolean) (SweepResult :type Hit%20Result%20Structure%20%28by%20ref%29))
  (Utilities|FlowControl|Sequence
    (:then_0
      (bind _asbp_first_person_character (Utilities|Casting|CastToBP_FirstPersonCharacter OtherActor))
      (if (Variables|Default|GetIsActive)
        (Variables|Default|SetIsActive false)
        (CallFunction|Slow)
        (Transformation|SetWorldScale3D (Variables|Default|GetStaticMesh) "0.700000,0.700000,0.700000")
        (Components|StaticMesh|SetStaticMesh (Variables|Default|GetStaticMesh) "/Game/Meshes/trap3.trap3")
        (Utilities|FlowControl|Delay 2.0)
        (Utilities|Time|ClearandInvalidateTimerbyHandle (stale Custom|Slow _returnvalue))
        (Variables|/Script/Engine.CharacterMovementComponent|SetMaxWalkSpeed (Variables|/Script/Engine.Character|GetCharacterMovement _asbp_first_person_character) 6e+02)
        (Variables|/Game/FirstPerson/Blueprints/BP_FirstPersonCharacter.BP_FirstPersonCharacter_C|SetA _asbp_first_person_character false)
        (Variables|/Script/Engine.CharacterMovementComponent|SetJumpZVelocity (Variables|/Script/Engine.Character|GetCharacterMovement _asbp_first_person_character) 6.5e+02)))
    (:then_1
      (Utilities|Casting|CastToBP_Fireball OtherActor)
      (Variables|Default|SetIsActive false)
      (Transformation|SetWorldScale3D (Variables|Default|GetStaticMesh) "0.700000,0.700000,0.700000")
      (Components|StaticMesh|SetStaticMesh (Variables|Default|GetStaticMesh) "/Game/Meshes/trap3.trap3"))))

(event Custom|Slow
  (bind _returnvalue (Utilities|Time|SetTimerbyEvent (delegate Custom|Slow) 0.1 true))
  (Variables|/Script/Engine.CharacterMovementComponent|SetMaxWalkSpeed (Variables|/Script/Engine.Character|GetCharacterMovement (stale OnComponentBeginOverlap(Sphere) _asbp_first_person_character)) 1.0)
  (Variables|/Game/FirstPerson/Blueprints/BP_FirstPersonCharacter.BP_FirstPersonCharacter_C|SetA (stale OnComponentBeginOverlap(Sphere) _asbp_first_person_character) true)
  (Variables|/Script/Engine.CharacterMovementComponent|SetJumpZVelocity (Variables|/Script/Engine.Character|GetCharacterMovement (stale OnComponentBeginOverlap(Sphere) _asbp_first_person_character)) 0.0))

(event EventBeginPlay)

(event Collision|EventActorBeginOverlap
  (params (OtherActor :type Actor%20Object%20Reference)))

(event EventTick
  (params (DeltaSeconds :type Float%20%28single-precision%29)))

(fn ConstructionScript)