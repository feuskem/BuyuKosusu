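; BP_TutorialTriggers is a trigger actor that shows the W_Tutorial widget when the first-person character overlaps it.
; On BeginPlay it requests a load message from the game instance, and LoadData copies the TUT1 save flag into Tutorial1Seen.
; The overlap skips the widget if that flag is set, and PressedAlready limits it to one display per instance.
; SaveData is empty, so this actor never writes the seen flag itself.
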(event EventBeginPlay
  (Class|BPIPersistence|RequestLoad(Message) (Game|GetGameInstance) self))

(event Collision|EventActorBeginOverlap
  (params (OtherActor :type Actor%20Object%20Reference))
  (Utilities|Casting|CastToBP_FirstPersonCharacter OtherActor)
  (if (not (Variables|Default|GetTutorial1Seen))
    (if (not (Variables|Default|GetPressedAlready))
      (bind _returnvalue (UserInterface|CreateWidget "/Game/W_Tutorial.W_Tutorial_C" (Game|GetPlayerController 0)))
      (UserInterface|Viewport|AddtoViewport _returnvalue 0)
      (Variables|Default|SetPressedAlready true))))

(event EventTick
  (params (DeltaSeconds :type Float%20%28single-precision%29)))

(event EventLoadData
  (params (SaveGameRef :type BP%20Save%20Game%20Object%20Reference))
  (Variables|Default|SetTutorial1Seen (Variables|/Game/Blueprints/BP_SaveGame.BP_SaveGame_C|GetTUT1 SaveGameRef)))

(event EventSaveData
  (params (SaveGameRef :type BP%20Save%20Game%20Object%20Reference)))

(fn ConstructionScript)