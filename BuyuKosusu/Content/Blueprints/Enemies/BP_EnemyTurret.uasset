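; Enemy cannon turret that shoots projectiles at the player and reports its death to BP_ObjectiveManager.
; A range sphere sets the AIC_Turret blackboard attack flag, while separate events fire and aim, leading the player by velocity and distance.
; Fireballs and daggers reduce health with color and scale feedback; deflected projectiles kill instantly and count as unique kills.
; Death unpossesses, poofs and destroys it; Mark briefly shows a highlight.
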(event OnSeePawn(PawnSensing)
  (params (Pawn :type Pawn%20Object%20Reference)))

(event OnComponentBeginOverlap(Sphere)
  (params (OverlappedComponent :type Primitive%20Component%20Object%20Reference) (OtherActor :type Actor%20Object%20Reference) (OtherComp :type Primitive%20Component%20Object%20Reference) (OtherBodyIndex :type Integer) (bFromSweep :type Boolean) (SweepResult :type Hit%20Result%20Structure%20%28by%20ref%29))
  (bind _self self)
  (bind _returnvalue (AI|GetAIController _self))
  (bind _asaic_turret (Utilities|Casting|CastToAIC_Turret _returnvalue))
  (bind _returnvalue_2 (AI|GetBlackboard _asaic_turret))
  (Utilities|Casting|CastToBP_FirstPersonCharacter OtherActor)
  (Variables|Default|SetWHY true)
  (Utilities|IsValid _returnvalue_2
    (:Is%20Valid
      (AI|Components|Blackboard|SetValueasBool _returnvalue_2 (Utilities|Name|MakeLiteralName "CannonCanAttack") true))))

(event OnComponentEndOverlap(Sphere)
  (params (OverlappedComponent :type Primitive%20Component%20Object%20Reference) (OtherActor :type Actor%20Object%20Reference) (OtherComp :type Primitive%20Component%20Object%20Reference) (OtherBodyIndex :type Integer))
  (bind _returnvalue (AI|GetBlackboard 0))
  (Utilities|Casting|CastToBP_FirstPersonCharacter OtherActor)
  (Utilities|IsValid _returnvalue
    (:Is%20Valid
      (Variables|Default|SetWHY false)
      (AI|Components|Blackboard|SetValueasBool _returnvalue (Utilities|Name|MakeLiteralName "CannonCanAttack") false))))

(event OnComponentBeginOverlap(Sphere1)
  (params (OverlappedComponent :type Primitive%20Component%20Object%20Reference) (OtherActor :type Actor%20Object%20Reference) (OtherComp :type Primitive%20Component%20Object%20Reference) (OtherBodyIndex :type Integer) (bFromSweep :type Boolean) (SweepResult :type Hit%20Result%20Structure%20%28by%20ref%29))
  (bind _health (Variables|Default|GetHealth))
  (Utilities|FlowControl|Sequence
    (:then_0
      (bind _asbp_projectile_deflect (Utilities|Casting|CastToBP_Projectile_Deflect OtherActor))
      (bind _result (Math|Integer|IncrementInt (Variables|/Game/FirstPerson/Blueprints/BP_FirstPersonCharacter.BP_FirstPersonCharacter_C|GetUniqueKills (stale EventBeginPlay _output_get)))
        (:%20%20
          (Variables|/Game/FirstPerson/Blueprints/BP_FirstPersonCharacter.BP_FirstPersonCharacter_C|SetUniqueKills (stale EventBeginPlay _output_get) _result)
          (Actor|DestroyActor _asbp_projectile_deflect)
          (CallFunction|Die :!label _label))))
    (:then_1
      (bind _asbp_fireball (Utilities|Casting|CastToBP_Fireball OtherActor))
      (Math|Integer|DecrementInt _health :!label _label_2
        (:%20%20
          (Utilities|IsValid _asbp_fireball
            (:Is%20Valid
              (Actor|DestroyActor _asbp_fireball))
            (:Is%20Not%20Valid
              (Actor|DestroyActor (stale _asbp_dagger))))
          (if (<= _health 0)
            (goto _label)
            (else
              (CallFunction|Damagedcolor)
              (bind _newtrack_0 (Timeline|Timeline_3 PlayFromStart)
                (:Update
                  (Transformation|SetWorldScale3D (Variables|Default|GetGun) (Math|Vector|MakeVector (* (.x (Math|Conversions|ToVector(Float) _newtrack_0)) -1.0) (.y (Math|Conversions|ToVector(Float) _newtrack_0)) (.z (Math|Conversions|ToVector(Float) _newtrack_0)))))
                (:Finished
                  (bind _newtrack_0_2 (Timeline|Timeline_4 PlayFromStart)
                    (:Update
                      (Transformation|SetWorldScale3D (Variables|Default|GetGun) (Math|Vector|MakeVector (* (.x (Math|Conversions|ToVector(Float) _newtrack_0_2)) -1.0) (.y (Math|Conversions|ToVector(Float) _newtrack_0_2)) (.z (Math|Conversions|ToVector(Float) _newtrack_0_2)))))
                    (:Finished
                      (CallFunction|NormalColor))))))))))
    (:then_2
      (bind _asbp_dagger (Utilities|Casting|CastToBP_Dagger OtherActor))
      (goto _label_2))))

(event Custom|FındRotation
  (bind _as_bp_first_person_character (Variables|Default|GetAs%20BP%20First%20Person%20Character))
  (bind _newtrack_0 (Timeline|Timeline PlayFromStart)
    (:Update
      (Utilities|FlowControl|Sequence
        (:then_0
          (Transformation|SetWorldRotation (Variables|Default|GetGun) (Math|Rotator|MakeRotator (.roll (Math|Rotator|Lerp(Rotator) (Transformation|GetActorRotation) (Math|Rotator|FindLookatRotation (Variables|Default|GetRotationStart) (+ (Transformation|GetActorLocation _as_bp_first_person_character) (* (* (/ (Math|Vector|VectorLength (- (Transformation|GetActorLocation _as_bp_first_person_character) (Transformation|GetActorLocation))) 2.2e+03) (Variables|/Script/Engine.MovementComponent|GetVelocity (Variables|/Script/Engine.Character|GetCharacterMovement _as_bp_first_person_character))) 0.8))) _newtrack_0 true)) (- (.pitch (Math|Rotator|Lerp(Rotator) (Transformation|GetActorRotation) (Math|Rotator|FindLookatRotation (Variables|Default|GetRotationStart) (+ (Transformation|GetActorLocation _as_bp_first_person_character) (* (* (/ (Math|Vector|VectorLength (- (Transformation|GetActorLocation _as_bp_first_person_character) (Transformation|GetActorLocation))) 2.2e+03) (Variables|/Script/Engine.MovementComponent|GetVelocity (Variables|/Script/Engine.Character|GetCharacterMovement _as_bp_first_person_character))) 0.8))) _newtrack_0 true)) 7.5) (.yaw (Math|Rotator|Lerp(Rotator) (Transformation|GetActorRotation) (Math|Rotator|FindLookatRotation (Variables|Default|GetRotationStart) (+ (Transformation|GetActorLocation _as_bp_first_person_character) (* (* (/ (Math|Vector|VectorLength (- (Transformation|GetActorLocation _as_bp_first_person_character) (Transformation|GetActorLocation))) 2.2e+03) (Variables|/Script/Engine.MovementComponent|GetVelocity (Variables|/Script/Engine.Character|GetCharacterMovement _as_bp_first_person_character))) 0.8))) _newtrack_0 true))) false false)
          (Variables|Default|SetRotationStart (Transformation|GetWorldLocation (Variables|Default|GetBase))))
        (:then_1
          (Transformation|SetWorldRotation (Variables|Default|GetBase) (Math|Rotator|MakeRotator 0.0 0.0 (.yaw (Math|Rotator|Lerp(Rotator) (Transformation|GetActorRotation) (Math|Rotator|FindLookatRotation (Variables|Default|GetRotationStart) (+ (Transformation|GetActorLocation _as_bp_first_person_character) (* (* (/ (Math|Vector|VectorLength (- (Transformation|GetActorLocation _as_bp_first_person_character) (Transformation|GetActorLocation))) 2.2e+03) (Variables|/Script/Engine.MovementComponent|GetVelocity (Variables|/Script/Engine.Character|GetCharacterMovement _as_bp_first_person_character))) 0.8))) _newtrack_0 true))) false false))
        (:then_2
          (Transformation|SetActorRotation (Math|Rotator|MakeRotator 0.0 (.pitch (Math|Rotator|Lerp(Rotator) (Transformation|GetActorRotation) (Math|Rotator|FindLookatRotation (Variables|Default|GetRotationStart) (+ (Transformation|GetActorLocation _as_bp_first_person_character) (* (* (/ (Math|Vector|VectorLength (- (Transformation|GetActorLocation _as_bp_first_person_character) (Transformation|GetActorLocation))) 2.2e+03) (Variables|/Script/Engine.MovementComponent|GetVelocity (Variables|/Script/Engine.Character|GetCharacterMovement _as_bp_first_person_character))) 0.8))) _newtrack_0 true)) (.yaw (Math|Rotator|Lerp(Rotator) (Transformation|GetActorRotation) (Math|Rotator|FindLookatRotation (Variables|Default|GetRotationStart) (+ (Transformation|GetActorLocation _as_bp_first_person_character) (* (* (/ (Math|Vector|VectorLength (- (Transformation|GetActorLocation _as_bp_first_person_character) (Transformation|GetActorLocation))) 2.2e+03) (Variables|/Script/Engine.MovementComponent|GetVelocity (Variables|/Script/Engine.Character|GetCharacterMovement _as_bp_first_person_character))) 0.8))) _newtrack_0 true)))))))))

(event Custom|Die
  (bind _manager (Variables|Default|GetManager))
  (Rendering|SetVisibility (Variables|Default|GetN_Poof) true false)
  (bind _asaic_turret (Utilities|Casting|CastToAIC_Turret (AI|GetAIController self)))
  (Pawn|UnPossess _asaic_turret)
  (Components|Activation|SetActive (Variables|Default|GetN_Poof) true true)
  (bind _result (Math|Integer|IncrementInt (Variables|/Game/Blueprints/BP_ObjectiveManager.BP_ObjectiveManager_C|GetEnemyCurrentAmount _manager))
    (:%20%20
      (Variables|/Game/Blueprints/BP_ObjectiveManager.BP_ObjectiveManager_C|SetEnemyCurrentAmount _manager _result)
      (CallFunction|Damagedcolor)
      (bind _newtrack_0 (Timeline|Timeline_1 PlayFromStart)
        (:Update
          (Transformation|SetWorldScale3D (Variables|Default|GetGun) (Math|Vector|MakeVector (* (.x (Math|Conversions|ToVector(Float) _newtrack_0)) -1.0) (.y (Math|Conversions|ToVector(Float) _newtrack_0)) (.z (Math|Conversions|ToVector(Float) _newtrack_0))))
          (Utilities|FlowControl|Delay 0.2)
          (Rendering|SetVisibility (Variables|Default|GetBase) false false)
          (Rendering|SetVisibility (Variables|Default|GetGun) false false)
          (Utilities|FlowControl|Delay 1.0)
          (Actor|DestroyActor))))))

(event Custom|AttackToPlayer
  (bind _arrow (Variables|Default|GetArrow))
  (bind _returnvalue (Transformation|GetWorldTransform _arrow))
  (Game|SpawnActorfromClass "/Game/Blueprints/BP_Projectile_Child.BP_Projectile_Child_C" (Math|Transform|MakeTransform (.location _returnvalue) (Math|Rotator|MakeRotator (.roll (.rotation _returnvalue)) (.pitch (.rotation _returnvalue)) (.yaw (.rotation _returnvalue))) "5.000000,5.000000,5.000000") "Undefined" "MultiplyWithRoot" 0 0))

(event EventBeginPlay
  (bind _asbp_first_person_character (Utilities|Casting|CastToBP_FirstPersonCharacter (Game|Player|GetPlayerPawn 0)))
  (bind _output_get (Variables|Default|SetAs%20BP%20First%20Person%20Character _asbp_first_person_character))
  (Variables|Default|SetRotationStart (Transformation|GetActorLocation))
  (Rendering|SetVisibility (Variables|Default|GetN_Poof) false false)
  (Rendering|SetVisibility (Variables|Default|GetLight) false false)
  (bind _returnvalue (Rendering|Material|CreateDynamicMaterialInstance (Variables|Default|GetLight) 0 "/Game/M_Bun2.M_Bun2" "None" :!class /Script/Engine.PrimitiveComponent))
  (Variables|Default|SetMaterial _returnvalue)
  (bind _returnvalue_2 (Actor|GetActorOfClass "/Game/Blueprints/BP_ObjectiveManager.BP_ObjectiveManager_C"))
  (Variables|Default|SetManager _returnvalue_2))

(event Collision|EventActorBeginOverlap
  (params (OtherActor :type Actor%20Object%20Reference)))

(event EventTick
  (params (DeltaSeconds :type Float%20%28single-precision%29)))

(event EventMark
  (Rendering|SetVisibility (Variables|Default|GetLight) true false)
  (bind _newtrack_0 (Timeline|Timeline_0 PlayFromStart)
    (:Update
      (Rendering|Material|SetScalarParameterValue (Variables|Default|GetMaterial) "OpacityValue" _newtrack_0 :!class /Script/Engine.MaterialInstanceDynamic))
    (:Finished
      (Rendering|SetVisibility (Variables|Default|GetLight) false false))))

(fn ConstructionScript)

(fn Damagedcolor
  (bind _gun (Variables|Default|GetGun))
  (bind _base (Variables|Default|GetBase))
  (Rendering|Material|SetMaterial _base 0 "/Game/Meshes/wands/materials/firecrystalasa.firecrystalasa")
  (Rendering|Material|SetMaterial _base 1 "/Game/Meshes/wands/materials/firecrystalasa.firecrystalasa")
  (Rendering|Material|SetMaterial _base 2 "/Game/Meshes/wands/materials/firecrystalasa.firecrystalasa")
  (Rendering|Material|SetMaterial _base 3 "/Game/Meshes/wands/materials/firecrystalasa.firecrystalasa")
  (Rendering|Material|SetMaterial _base 4 "/Game/Meshes/wands/materials/firecrystalasa.firecrystalasa")
  (Rendering|Material|SetMaterial _gun 0 "/Game/Meshes/wands/materials/firecrystalasa.firecrystalasa")
  (Rendering|Material|SetMaterial _gun 1 "/Game/Meshes/wands/materials/firecrystalasa.firecrystalasa")
  (Rendering|Material|SetMaterial _gun 2 "/Game/Meshes/wands/materials/firecrystalasa.firecrystalasa")
  (Rendering|Material|SetMaterial _gun 3 "/Game/Meshes/wands/materials/firecrystalasa.firecrystalasa"))

(fn NormalColor
  (bind _base (Variables|Default|GetBase))
  (bind _gun (Variables|Default|GetGun))
  (Rendering|Material|SetMaterial _base 0 "/Game/Meshes/cannon__cannonball__bomb/newcannonmaterails/cannonholder.cannonholder")
  (Rendering|Material|SetMaterial _base 2 "/Game/Meshes/cannon__cannonball__bomb/newcannonmaterails/cannonholder_001.cannonholder_001")
  (Rendering|Material|SetMaterial _base 3 "/Game/Meshes/cannon__cannonball__bomb/newcannonmaterails/cannonwood_001.cannonwood_001")
  (Rendering|Material|SetMaterial _base 4 "/Game/Meshes/cannon__cannonball__bomb/newcannonmaterails/cannonwheels.cannonwheels")
  (Rendering|Material|SetMaterial _base 5 "/Game/Meshes/cannon__cannonball__bomb/newcannonmaterails/cannonwood_002.cannonwood_002")
  (Rendering|Material|SetMaterial _gun 0 "/Game/Meshes/cannon__cannonball__bomb/newcannonmaterails/cannonround.cannonround")
  (Rendering|Material|SetMaterial _gun 1 "/Game/Meshes/cannon__cannonball__bomb/newcannonmaterails/cannonround_001.cannonround_001")
  (Rendering|Material|SetMaterial _gun 2 "/Game/Meshes/cannon__cannonball__bomb/newcannonmaterails/cannonrope_001.cannonrope_001")
  (Rendering|Material|SetMaterial _gun 3 "/Game/Meshes/cannon__cannonball__bomb/newcannonmaterails/CannonInsideYellow.CannonInsideYellow"))