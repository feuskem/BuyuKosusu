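; Flying fairy enemy that drifts toward random points near its StaticMesh component and fires projectiles.
; Each tick it moves and turns to lead the player using velocity and distance; range overlaps update a Blackboard flag, and Attack spawns projectiles with a cooldown.
; Fireballs and daggers decrement health with a material/scale hit flash, while deflected projectiles kill outright.
; Death updates BP_ObjectiveManager's count; Mark briefly shows an animated highlight.
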(event OnComponentBeginOverlap(r)
  (params (OverlappedComponent :type Primitive%20Component%20Object%20Reference) (OtherActor :type Actor%20Object%20Reference) (OtherComp :type Primitive%20Component%20Object%20Reference) (OtherBodyIndex :type Integer) (bFromSweep :type Boolean) (SweepResult :type Hit%20Result%20Structure%20%28by%20ref%29))
  (bind _returnvalue (AI|GetBlackboard 0))
  (Utilities|Casting|CastToBP_FirstPersonCharacter OtherActor)
  (Utilities|IsValid _returnvalue
    (:Is%20Valid
      (AI|Components|Blackboard|SetValueasBool _returnvalue (Utilities|Name|MakeLiteralName "IsPlayerInRange") true))))

(event OnComponentEndOverlap(r)
  (params (OverlappedComponent :type Primitive%20Component%20Object%20Reference) (OtherActor :type Actor%20Object%20Reference) (OtherComp :type Primitive%20Component%20Object%20Reference) (OtherBodyIndex :type Integer))
  (bind _returnvalue (AI|GetBlackboard 0))
  (Utilities|Casting|CastToBP_FirstPersonCharacter OtherActor)
  (Utilities|IsValid _returnvalue
    (:Is%20Valid
      (AI|Components|Blackboard|SetValueasBool _returnvalue (Utilities|Name|MakeLiteralName "IsPlayerInRange") false))))

(event OnComponentBeginOverlap(CapsuleComponent)
  (params (OverlappedComponent :type Primitive%20Component%20Object%20Reference) (OtherActor :type Actor%20Object%20Reference) (OtherComp :type Primitive%20Component%20Object%20Reference) (OtherBodyIndex :type Integer) (bFromSweep :type Boolean) (SweepResult :type Hit%20Result%20Structure%20%28by%20ref%29))
  (bind _mesh (Variables|Character|GetMesh))
  (bind _mesh_2 (Variables|Character|GetMesh))
  (bind _mesh_3 (Variables|Character|GetMesh))
  (bind _mesh_4 (Variables|Character|GetMesh))
  (bind _objectivemanager_0 (Variables|Default|GetObjectiveManager_0))
  (Utilities|FlowControl|Sequence
    (:then_0
      (bind _asbp_fireball (Utilities|Casting|CastToBP_Fireball OtherActor))
      (bind _result (Math|Integer|DecrementInt (Variables|Default|GetHealth) :!label _label)
        (:%20%20
          (Variables|Default|SetHealth _result)
          (Utilities|IsValid _asbp_fireball
            (:Is%20Valid
              (Actor|DestroyActor _asbp_fireball))
            (:Is%20Not%20Valid
              (Utilities|IsValid (stale _asbp_dagger)
                (:Is%20Valid
                  (Actor|DestroyActor (stale _asbp_dagger)))))))))
    (:then_1
      (bind _asbp_dagger (Utilities|Casting|CastToBP_Dagger OtherActor))
      (goto _label))
    (:then_2
      (bind _asbp_projectile_flying_deflect (Utilities|Casting|CastToBP_Projectile_FlyingDeflect OtherActor))
      (Development|PrintString "AHEE")
      (Variables|Default|SetHealth 0)
      (Utilities|IsValid _asbp_projectile_flying_deflect
        (:Is%20Valid
          (Actor|DestroyActor _asbp_projectile_flying_deflect))
        (:Is%20Not%20Valid
          _))))
  (if (<= (Variables|Default|GetHealth) 0)
    (Rendering|Material|SetMaterial _mesh_3 0 "/Game/Meshes/wands/materials/firecrystalasa.firecrystalasa")
    (Rendering|Material|SetMaterial _mesh_3 1 "/Game/Meshes/wands/materials/firecrystalasa.firecrystalasa")
    (Rendering|Material|SetMaterial _mesh_3 2 "/Game/Meshes/wands/materials/firecrystalasa.firecrystalasa")
    (Rendering|Material|SetMaterial _mesh_3 3 "/Game/Meshes/wands/materials/firecrystalasa.firecrystalasa")
    (Rendering|Material|SetMaterial _mesh_3 4 "/Game/Meshes/wands/materials/firecrystalasa.firecrystalasa")
    (Rendering|Material|SetMaterial _mesh_3 5 "/Game/Meshes/wands/materials/firecrystalasa.firecrystalasa")
    (bind _newtrack_0 (Timeline|Timeline_6 PlayFromStart)
      (:Update
        (Transformation|SetWorldScale3D (Variables|Character|GetMesh) (Math|Conversions|ToVector(Float) _newtrack_0))
        (Components|Activation|SetActive (Variables|Default|GetNiagara) true false)
        (Utilities|FlowControl|Delay 1.0)
        (if (Variables|Default|GetYEEP)
          _
          (else
            (bind _result_2 (Math|Integer|IncrementInt (Variables|/Game/Blueprints/BP_ObjectiveManager.BP_ObjectiveManager_C|GetEnemyCurrentAmount _objectivemanager_0))
              (:%20%20
                (Variables|/Game/Blueprints/BP_ObjectiveManager.BP_ObjectiveManager_C|SetEnemyCurrentAmount _objectivemanager_0 _result_2)
                (Variables|Default|SetYEEP true)))))
        (Actor|DestroyActor)))
    (else
      (Rendering|Material|SetMaterial _mesh_4 0 "/Game/Meshes/wands/materials/firecrystalasa.firecrystalasa")
      (Rendering|Material|SetMaterial _mesh_4 1 "/Game/Meshes/wands/materials/firecrystalasa.firecrystalasa")
      (Rendering|Material|SetMaterial _mesh_4 2 "/Game/Meshes/wands/materials/firecrystalasa.firecrystalasa")
      (Rendering|Material|SetMaterial _mesh_4 3 "/Game/Meshes/wands/materials/firecrystalasa.firecrystalasa")
      (Rendering|Material|SetMaterial _mesh_4 4 "/Game/Meshes/wands/materials/firecrystalasa.firecrystalasa")
      (Rendering|Material|SetMaterial _mesh_4 5 "/Game/Meshes/wands/materials/firecrystalasa.firecrystalasa")
      (bind _newtrack_0_2 (Timeline|Timeline_8 PlayFromStart)
        (:Update
          (Transformation|SetWorldScale3D _mesh (Math|Conversions|ToVector(Float) _newtrack_0_2)))
        (:Finished
          (bind _newtrack_0_3 (Timeline|Timeline_9 PlayFromStart)
            (:Update
              (Transformation|SetWorldScale3D _mesh (Math|Conversions|ToVector(Float) _newtrack_0_3)))
            (:Finished
              (Rendering|Material|SetMaterial _mesh_2 0 "/Game/Meshes/WispParts/BlenderMaterials/lambert3.lambert3")
              (Rendering|Material|SetMaterial _mesh_2 1 "/Game/Meshes/WispParts/BlenderMaterials/lambert2.lambert2")
              (Rendering|Material|SetMaterial _mesh_2 2 "/Game/Meshes/WispRIGGED/blendermaterials/lower_wing.lower_wing")
              (Rendering|Material|SetMaterial _mesh_2 3 "/Game/Meshes/WispParts/BlenderMaterials/eyes.eyes")
              (Rendering|Material|SetMaterial _mesh_2 4 "/Game/Meshes/WispParts/BlenderMaterials/lambert4.lambert4")
              (Rendering|Material|SetMaterial _mesh_2 5 "/Game/Meshes/WispParts/BlenderMaterials/fairy_wings.fairy_wings"))))))))

(event OnComponentBeginOverlap(Capsule)
  (params (OverlappedComponent :type Primitive%20Component%20Object%20Reference) (OtherActor :type Actor%20Object%20Reference) (OtherComp :type Primitive%20Component%20Object%20Reference) (OtherBodyIndex :type Integer) (bFromSweep :type Boolean) (SweepResult :type Hit%20Result%20Structure%20%28by%20ref%29)))

(event Custom|SetPoint
  (Transformation|SetActorLocation (Math|Interpolation|VInterpTo (Transformation|GetActorLocation) (Variables|Default|GetSetTarget%20Location) (Utilities|Time|GetWorldDeltaSeconds) 1.0) false false))

(event Custom|RotatePlayer
  (bind _as_bp_first_person_character_0 (Variables|Default|GetAs%20BP%20First%20Person%20Character_0))
  (bind _newtrack_0 (Timeline|Timeline_4_0 PlayFromStart)
    (:Update
      (Transformation|SetActorRotation (Math|Rotator|Lerp(Rotator) (Transformation|GetActorRotation) (Math|Rotator|FindLookatRotation (Variables|Default|GetRotationStart) (+ (Transformation|GetActorLocation _as_bp_first_person_character_0) (* (* (/ (Math|Vector|VectorLength (- (Transformation|GetActorLocation _as_bp_first_person_character_0) (Transformation|GetActorLocation))) 2.2e+03) (Variables|/Script/Engine.MovementComponent|GetVelocity (Variables|/Script/Engine.Character|GetCharacterMovement _as_bp_first_person_character_0))) 1.15))) _newtrack_0 true))
      (Variables|Default|SetRotationStart (Transformation|GetActorLocation)))))

(event Custom|Attack
  (bind _arrow1 (Variables|Default|GetArrow1))
  (bind _returnvalue (Transformation|GetWorldTransform _arrow1))
  (Game|SpawnActorfromClass "/Game/Blueprints/BP_Projectile_ChildFairy.BP_Projectile_ChildFairy_C" (Math|Transform|MakeTransform (.location _returnvalue) (.rotation _returnvalue) "5.000000,5.000000,5.000000") "Undefined" "MultiplyWithRoot" 0 0)
  (Variables|Default|SetCanAttack false)
  (Utilities|FlowControl|Delay (Variables|Default|GetAttackCooldown))
  (Variables|Default|SetCanAttack true))

(event Custom|ChangeRandomLocv
  (Variables|Default|SetSetTarget%20Location (Math|Random|RandomPointinBoundingBox (Variables|Default|GetBoxOrigin) "500.000000,500.000000,100.000000")))

(event EventBeginPlay
  (|CallParentFunction)
  (Utilities|FlowControl|Sequence
    (:then_0
      (bind _returnvalue (Actor|GetActorOfClass "/Game/Blueprints/BP_ObjectiveManager.BP_ObjectiveManager_C"))
      (Variables|Default|SetObjectiveManager_0 _returnvalue))
    (:then_1
      (Variables|Default|SetBoxOrigin (Transformation|GetWorldLocation (Variables|Default|GetStaticMesh)))
      (Variables|Default|SetBoxExtent (Components|Box|GetScaledBoxExtent (Variables|Default|GetBox_0)))
      (CallFunction|ChangeRandomLocv)
      (Rendering|SetVisibility (Variables|Default|GetLight) false false)
      (bind _returnvalue_2 (Rendering|Material|CreateDynamicMaterialInstance (Variables|Default|GetLight) 0 "/Game/M_Bun2.M_Bun2" "None" :!class /Script/Engine.PrimitiveComponent))
      (Variables|Default|SetMaterial_0 _returnvalue_2))
    (:then_2
      (bind _asbp_first_person_character (Utilities|Casting|CastToBP_FirstPersonCharacter (Game|Player|GetPlayerPawn 0)))
      (Variables|Default|SetAs%20BP%20First%20Person%20Character_0 _asbp_first_person_character))))

(event Collision|EventActorBeginOverlap
  (params (OtherActor :type Actor%20Object%20Reference))
  (|CallParentFunction OtherActor) ; This node is disabled and will not be called.\nDrag off pins to build functionality.
)

(event EventTick
  (params (DeltaSeconds :type Float%20%28single-precision%29))
  (|CallParentFunction DeltaSeconds)
  (CallFunction|RotatePlayer)
  (CallFunction|SetPoint))

(event EventAttacktoPlayer
  (|CallParentFunction))

(event EventMark
  (Rendering|SetVisibility (Variables|Default|GetLight) true false)
  (bind _newtrack_0 (Timeline|Timeline_5 PlayFromStart)
    (:Update
      (Rendering|Material|SetScalarParameterValue (Variables|Default|GetMaterial_0) "OpacityValue" _newtrack_0 :!class /Script/Engine.MaterialInstanceDynamic))
    (:Finished
      (Rendering|SetVisibility (Variables|Default|GetLight) false false))))

(fn ConstructionScript
  (|CallParentFunction))