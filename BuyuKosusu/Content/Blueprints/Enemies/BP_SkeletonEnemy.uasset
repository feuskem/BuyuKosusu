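; Skeleton bomber enemy that chases the player and damages them on contact, destroying itself.
; A detection overlap writes the target and in-range flag to the AIC_Skeleton blackboard and toggles a small fire effect.
; Fireball and dagger hits share a health decrement; death plays Niagara, unpossesses, hides meshes, then destroys the actor.
; A Mark event briefly shows a highlight, animating its dynamic material's opacity through a timeline.
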(event OnComponentBeginOverlap(DetectPlayer)
  (params (OverlappedComponent :type Primitive%20Component%20Object%20Reference) (OtherActor :type Actor%20Object%20Reference) (OtherComp :type Primitive%20Component%20Object%20Reference) (OtherBodyIndex :type Integer) (bFromSweep :type Boolean) (SweepResult :type Hit%20Result%20Structure%20%28by%20ref%29))
  (bind _self self)
  (bind _returnvalue (AI|GetAIController _self))
  (bind _asaic_skeleton (Utilities|Casting|CastToAIC_Skeleton _returnvalue))
  (bind _returnvalue_2 (AI|GetBlackboard _asaic_skeleton))
  (bind _asbp_first_person_character (Utilities|Casting|CastToBP_FirstPersonCharacter OtherActor))
  (Variables|Default|SetIsChasing true)
  (Utilities|IsValid _returnvalue_2
    (:Is%20Valid
      (AI|Components|Blackboard|SetValueasObject _returnvalue_2 (Utilities|Name|MakeLiteralName "TargetActor") _asbp_first_person_character)
      (AI|Components|Blackboard|SetValueasBool _returnvalue_2 (Utilities|Name|MakeLiteralName "IsPlayerInRange") true)
      (Rendering|SetVisibility (Variables|Default|GetP_Fire_Small) true false))))

(event OnComponentEndOverlap(DetectPlayer)
  (params (OverlappedComponent :type Primitive%20Component%20Object%20Reference) (OtherActor :type Actor%20Object%20Reference) (OtherComp :type Primitive%20Component%20Object%20Reference) (OtherBodyIndex :type Integer))
  (bind _self self)
  (bind _returnvalue (AI|GetAIController _self))
  (bind _asaic_skeleton (Utilities|Casting|CastToAIC_Skeleton _returnvalue))
  (bind _returnvalue_2 (AI|GetBlackboard _asaic_skeleton))
  (Utilities|Casting|CastToBP_FirstPersonCharacter OtherActor)
  (Variables|Default|SetIsChasing false)
  (Utilities|IsValid _returnvalue_2
    (:Is%20Valid
      (AI|Components|Blackboard|ClearValue _returnvalue_2 (Utilities|Name|MakeLiteralName "TargetActor"))
      (AI|Components|Blackboard|SetValueasBool _returnvalue_2 (Utilities|Name|MakeLiteralName "IsPlayerInRange") false)
      (Rendering|SetVisibility (Variables|Default|GetP_Fire_Small) false false))))

(event OnComponentBeginOverlap(Sphere)
  (params (OverlappedComponent :type Primitive%20Component%20Object%20Reference) (OtherActor :type Actor%20Object%20Reference) (OtherComp :type Primitive%20Component%20Object%20Reference) (OtherBodyIndex :type Integer) (bFromSweep :type Boolean) (SweepResult :type Hit%20Result%20Structure%20%28by%20ref%29))
  (bind _asbp_first_person_character (Utilities|Casting|CastToBP_FirstPersonCharacter OtherActor))
  (Actor|DestroyActor)
  (Variables|/Game/FirstPerson/Blueprints/BP_FirstPersonCharacter.BP_FirstPersonCharacter_C|SetHealth _asbp_first_person_character (- (Variables|/Game/FirstPerson/Blueprints/BP_FirstPersonCharacter.BP_FirstPersonCharacter_C|GetHealth _asbp_first_person_character) 3e+01)))

(event OnComponentBeginOverlap(CapsuleComponent)
  (params (OverlappedComponent :type Primitive%20Component%20Object%20Reference) (OtherActor :type Actor%20Object%20Reference) (OtherComp :type Primitive%20Component%20Object%20Reference) (OtherBodyIndex :type Integer) (bFromSweep :type Boolean) (SweepResult :type Hit%20Result%20Structure%20%28by%20ref%29))
  (Utilities|FlowControl|Sequence
    (:then_0
      (bind _asbp_fireball (Utilities|Casting|CastToBP_Fireball OtherActor))
      (Actor|DestroyActor _asbp_fireball))
    (:then_1
      (bind _asbp_dagger (Utilities|Casting|CastToBP_Dagger OtherActor))
      (Actor|DestroyActor _asbp_dagger)))
  (Math|Integer|DecrementInt (Variables|Default|GetEnemyhealth)
    (:%20%20
      (if (<= (Variables|Default|GetEnemyhealth) 0)
        (Components|Activation|Activate (Variables|Default|GetNiagara) true)
        (Pawn|UnPossess (AI|GetAIController self))
        (Utilities|FlowControl|Delay 0.4)
        (Development|SetHiddeninGame (Variables|Character|GetMesh) true false)
        (Utilities|FlowControl|Delay 0.4)
        (Actor|DestroyActor)))))

(event EventBeginPlay
  (Components|Activation|Deactivate (Variables|Default|GetNiagara))
  (Rendering|SetVisibility (Variables|Default|GetLight) false false)
  (bind _returnvalue (Rendering|Material|CreateDynamicMaterialInstance (Variables|Default|GetLight) 0 "/Game/M_Bun2.M_Bun2" "None" :!class /Script/Engine.PrimitiveComponent))
  (Variables|Default|SetMaterial _returnvalue))

(event Collision|EventActorBeginOverlap
  (params (OtherActor :type Actor%20Object%20Reference)))

(event EventTick
  (params (DeltaSeconds :type Float%20%28single-precision%29)))

(event EventMark
  (Rendering|SetVisibility (Variables|Default|GetLight) true false)
  (bind _newtrack_0 (Timeline|Timeline PlayFromStart)
    (:Update
      (Rendering|Material|SetScalarParameterValue (Variables|Default|GetMaterial) "OpacityValue" _newtrack_0 :!class /Script/Engine.MaterialInstanceDynamic))
    (:Finished
      (Rendering|SetVisibility (Variables|Default|GetLight) false false))))

(fn ConstructionScript)