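; Water enemy that fires projectiles at the player, dives when damaged, and resurfaces at a random navmesh point near its spawn.
; Overlaps only set AIC_Water blackboard flags: ice stuns, fireballs and daggers register hits; action events are exposed for outside callers.
; Timelines drive diving, relocation, turning toward the player, a stun lift that drops Health to one, and a fading mark highlight.
; Death plays Niagara, unpossesses and destroys it.
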(event OnComponentBeginOverlap(CapsuleComponent)
  (params (OverlappedComponent :type Primitive%20Component%20Object%20Reference) (OtherActor :type Actor%20Object%20Reference) (OtherComp :type Primitive%20Component%20Object%20Reference) (OtherBodyIndex :type Integer) (bFromSweep :type Boolean) (SweepResult :type Hit%20Result%20Structure%20%28by%20ref%29))
  (bind _self self)
  (bind _returnvalue (AI|GetAIController _self))
  (bind _returnvalue_2 (AI|GetBlackboard _returnvalue))
  (Utilities|FlowControl|Sequence
    (:then_0
      (Utilities|Casting|CastToBP_Ice OtherActor)
      (if (not (Variables|Default|GetIsStunned))
        (AI|Components|Blackboard|SetValueasBool (AI|GetBlackboard (AI|GetAIController self)) (Utilities|Name|MakeLiteralName "IsStunned") true)))
    (:then_1
      (Utilities|Casting|CastToBP_Fireball OtherActor)
      (Utilities|IsValid _returnvalue_2 :!label _label
        (:Is%20Valid
          (AI|Components|Blackboard|SetValueasBool _returnvalue_2 (Utilities|Name|MakeLiteralName "IsHit") true))))
    (:then_2
      (Utilities|Casting|CastToBP_Dagger OtherActor)
      (goto _label))))

(event Custom|TakeDamage
  (bind _result (Math|Integer|DecrementInt (Variables|Default|GetHealth))
    (:%20%20
      (if (> _result 0)
        (CallFunction|GoUnderWater)
        (else
          (CallFunction|Die))))))

(event Custom|GoUnderWater
  (bind _returnvalue (Transformation|GetActorLocation))
  (Variables|Default|SetIsUnderWater true)
  (Variables|Default|SetCanAttack false)
  (bind _newtrack_0 (Timeline|Timeline PlayFromStart)
    (:Update
      (Transformation|SetActorLocation (Math|Vector|MakeVector (.x _returnvalue) (.y _returnvalue) (- (.z _returnvalue) _newtrack_0)) false false))))

(event Custom|StartPopUpMovement
  (bind _returnvalue (Transformation|GetActorLocation))
  (AI|Components|Blackboard|SetValueasBool (AI|GetBlackboard (AI|GetAIController self)) (Utilities|Name|MakeLiteralName "IsHit") false)
  (Variables|Default|SetStartLocation _returnvalue)
  (bind _randomlocation (Class|NavigationSystemV1|GetRandomLocationinNavigableRadius _returnvalue 3.5e+02 0 0 :!label _label))
  (Variables|Default|SetTargetLocation (Math|Vector|MakeVector (.x _randomlocation) (.y _randomlocation) (.z (Transformation|GetActorLocation))))
  (if (and (>= (Math|Vector|VectorLength (- (Variables|Default|GetTargetLocation) (Variables|Default|GetStartLocation))) 2e+02) (<= (Math|Vector|VectorLength (- (Variables|Default|GetTargetLocation) (Variables|Default|GetPivotPosition))) 4.5e+02))
    (bind _alpha (Timeline|Timeline_0 PlayFromStart)
      (:Update
        (Transformation|SetActorLocation (Math|Vector|Lerp(Vector) (Variables|Default|GetStartLocation) (Variables|Default|GetTargetLocation) _alpha) false false))
      (:Finished
        (if (Variables|Default|GetIsUnderWater)
          (bind _newtrack_0 (Timeline|Timeline_1 PlayFromStart)
            (:Update
              (Transformation|SetActorLocation (Math|Vector|MakeVector (.x (Variables|Default|GetTargetLocation)) (.y (Variables|Default|GetTargetLocation)) (+ (.z (Transformation|GetActorLocation)) (* _newtrack_0 1.0))) false false))
            (:Finished
              (Variables|Default|SetIsPoppingUp true :!label _label_2)
              (Variables|Default|SetIsUnderWater false)))
          (else
            (goto _label_2)))
        (Variables|Default|SetStartLocation (Transformation|GetActorLocation))))
    (else
      (goto _label))))

(event Custom|AttackToPlayer
  (bind _arrow1 (Variables|Default|GetArrow1))
  (bind _returnvalue (Transformation|GetWorldTransform _arrow1))
  (Game|SpawnActorfromClass "/Game/Blueprints/BP_Projectile_Child.BP_Projectile_Child_C" (Math|Transform|MakeTransform (.location _returnvalue) (.rotation _returnvalue) "5.000000,5.000000,5.000000") "Undefined" "MultiplyWithRoot" 0 0)
  (Variables|Default|SetCanAttack false)
  (Utilities|FlowControl|Delay (Variables|Default|GetAttackCooldown))
  (Variables|Default|SetCanAttack true))

(event Custom|ApplyStun
  (bind _returnvalue (Transformation|GetActorLocation))
  (AI|Components|Blackboard|SetValueasBool (AI|GetBlackboard (AI|GetAIController self)) (Utilities|Name|MakeLiteralName "StunUsed") true)
  (Variables|Default|SetIsStunned true)
  (Variables|Default|SetHealth 1)
  (bind _newtrack_0 (Timeline|Timeline_2 PlayFromStart)
    (:Update
      (Transformation|SetActorLocation (Math|Vector|MakeVector (.x _returnvalue) (.y _returnvalue) (+ (.z _returnvalue) _newtrack_0)) false false)
      (Utilities|FlowControl|Delay 3.0)
      (CallFunction|RemoveStun))))

(event Custom|RemoveStun
  (bind _returnvalue (Transformation|GetActorLocation))
  (bind _newtrack_0 (Timeline|Timeline_3 PlayFromStart)
    (:Update
      (Transformation|SetActorLocation (Math|Vector|MakeVector (.x _returnvalue) (.y _returnvalue) (- (.z _returnvalue) _newtrack_0)) false false)
      (AI|Components|Blackboard|SetValueasBool (AI|GetBlackboard (AI|GetAIController self)) (Utilities|Name|MakeLiteralName "IsStunned") false)
      (AI|Components|Blackboard|SetValueasBool (AI|GetBlackboard (AI|GetAIController self)) (Utilities|Name|MakeLiteralName "StunUsed") false))
    (:Finished
      (Variables|Default|SetIsStunned false))))

(event Custom|FindLookAtRotation
  (bind _newtrack_0 (Timeline|Rotation PlayFromStart)
    (:Update
      (Transformation|SetActorRotation (Math|Rotator|Lerp(Rotator) (Transformation|GetActorRotation) (Math|Rotator|FindLookatRotation (Variables|Default|GetRotationStart) (Transformation|GetActorLocation (Variables|Default|GetAs%20BP%20First%20Person%20Character))) _newtrack_0 true))
      (Variables|Default|SetRotationStart (Transformation|GetActorLocation)))))

(event Custom|Die
  (bind _niagara (Variables|Default|GetNiagara))
  (Rendering|SetVisibility _niagara true false)
  (Components|Activation|Activate _niagara true)
  (bind _asaic_water (Utilities|Casting|CastToAIC_Water (AI|GetAIController self)))
  (Pawn|UnPossess _asaic_water)
  (Rendering|SetVisibility (Variables|Default|GetStaticMesh) false false)
  (Utilities|FlowControl|Delay 1.0)
  (Actor|DestroyActor))

(event EventBeginPlay
  (bind _returnvalue (Transformation|GetActorLocation))
  (Variables|Default|SetPivotPosition _returnvalue)
  (bind _asbp_first_person_character (Utilities|Casting|CastToBP_FirstPersonCharacter (Game|Player|GetPlayerPawn 0)))
  (Variables|Default|SetAs%20BP%20First%20Person%20Character _asbp_first_person_character)
  (Variables|Default|SetRotationStart _returnvalue)
  (Rendering|SetVisibility (Variables|Default|GetNiagara) false false)
  (Rendering|SetVisibility (Variables|Default|GetLight) false false)
  (bind _returnvalue_2 (Rendering|Material|CreateDynamicMaterialInstance (Variables|Default|GetLight) 0 "/Game/M_Bun2.M_Bun2" "None" :!class /Script/Engine.PrimitiveComponent))
  (Variables|Default|SetMaterial _returnvalue_2))

(event Collision|EventActorBeginOverlap
  (params (OtherActor :type Actor%20Object%20Reference)))

(event EventTick
  (params (DeltaSeconds :type Float%20%28single-precision%29)))

(event EventMark
  (Rendering|SetVisibility (Variables|Default|GetLight) true false)
  (bind _newtrack_0 (Timeline|Timeline_4 PlayFromStart)
    (:Update
      (Rendering|Material|SetScalarParameterValue (Variables|Default|GetMaterial) "OpacityValue" _newtrack_0 :!class /Script/Engine.MaterialInstanceDynamic))
    (:Finished
      (Rendering|SetVisibility (Variables|Default|GetLight) false false))))

(fn ConstructionScript)