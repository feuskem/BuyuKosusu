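; YANLISBU is an enemy actor that dives under the ground or water, relocates, pops up and fires projectiles.
; Timelines sink it, lerp it to a random navigable point at least 200 units away, then raise it if submerged.
; AttackToPlayer, not called in this graph, spawns a projectile, waits out a cooldown and relocates again.
; Damage decrements Health until destruction; stun sets Health to one, then sends it under when it expires.
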(event Custom|TakeDamage
  (bind _result (Math|Integer|DecrementInt (Variables|Default|GetHealth))
    (:%20%20
      (if (not (> _result 0))
        (Actor|DestroyActor)))))

(event Custom|GoUnderWater
  (bind _returnvalue (Transformation|GetActorLocation))
  (Variables|Default|SetIsUnderWater true)
  (Variables|Default|SetCanAttack false)
  (bind _newtrack_0 (Timeline|GoUnder PlayFromStart)
    (:Update
      (Transformation|SetActorLocation (Math|Vector|MakeVector (.x _returnvalue) (.y _returnvalue) (- (.z _returnvalue) _newtrack_0)) false false)
      (Utilities|FlowControl|Delay 1.5)
      (CallFunction|StartPopUpMovement))))

(event Custom|StartPopUpMovement
  (bind _returnvalue (Transformation|GetActorLocation))
  (Variables|Default|SetStartLocation _returnvalue)
  (bind _randomlocation (Class|NavigationSystemV1|GetRandomLocationinNavigableRadius _returnvalue 3.5e+02 0 0 :!label _label))
  (Variables|Default|SetTargetLocation (Math|Vector|MakeVector (.x _randomlocation) (.y _randomlocation) (.z (Transformation|GetActorLocation))))
  (if (>= (Math|Vector|VectorLength (- (Variables|Default|GetTargetLocation) (Variables|Default|GetStartLocation))) 2e+02)
    (bind _alpha (Timeline|PopUp PlayFromStart)
      (:Update
        (Transformation|SetActorLocation (Math|Vector|Lerp(Vector) (Variables|Default|GetStartLocation) (Variables|Default|GetTargetLocation) _alpha) false false))
      (:Finished
        (if (Variables|Default|GetIsUnderWater)
          (bind _newtrack_0 (Timeline|Timeline PlayFromStart)
            (:Update
              (Transformation|SetActorLocation (Math|Vector|MakeVector (.x (Variables|Default|GetTargetLocation)) (.y (Variables|Default|GetTargetLocation)) (+ (.z (Transformation|GetActorLocation)) (* _newtrack_0 1.0))) false false))
            (:Finished
              (Variables|Default|SetIsPoppingUp true :!label _label_2)
              (Variables|Default|SetIsUnderWater false)))
          (else
            (goto _label_2)))
        (Variables|Default|SetStartLocation (Transformation|GetActorLocation))))
    (else
      (goto _label))))

(event Custom|AttackToPlayer
  (Game|SpawnActorfromClass "/Game/Blueprints/BP_Projectile_Child.BP_Projectile_Child_C" (Transformation|GetWorldTransform (Variables|Default|GetArrow)) "Undefined" "MultiplyWithRoot" 0 0)
  (Variables|Default|SetCanAttack false)
  (Utilities|FlowControl|Delay (Variables|Default|GetAttackCooldown))
  (Variables|Default|SetCanAttack true)
  (CallFunction|StartPopUpMovement))

(event Custom|ApplyStun
  (Variables|Default|SetIsStunned true)
  (Variables|Default|SetHealth 1)
  (Utilities|FlowControl|Delay (Variables|Default|GetStunDuration))
  (CallFunction|RemoveStun))

(event Custom|RemoveStun
  (Variables|Default|SetIsStunned false)
  (CallFunction|GoUnderWater))

(event EventBeginPlay
  (Utilities|FlowControl|Delay 1.0)
  (CallFunction|GoUnderWater))

(event Collision|EventActorBeginOverlap
  (params (OtherActor :type Actor%20Object%20Reference)))

(event EventTick
  (params (DeltaSeconds :type Float%20%28single-precision%29)))

(fn ConstructionScript)