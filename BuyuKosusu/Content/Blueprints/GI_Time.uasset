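; GI_Time is a Game Instance that manages saving and loading through a single BP_SaveGame object in one slot.
; It creates or loads the save, writes it synchronously or asynchronously, and broadcasts when loading or saving finishes.
; Save requests pass all BPI_Saveable actors to the save object before writing to disk.
; Load requests have that object supply data to the requester without reading the slot again.
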(event Custom|SaveGame
  (params (Async :type Boolean))
  (if Async
    (|AsyncSaveGametoSlot (Variables|Default|GetSaveGameRef) (Variables|Default|GetSaveGameSlot)
      (:Completed
        (Default|CallGameSaved (Variables|Default|GetSaveGameRef))))
    (else
      (SaveGame|SaveGametoSlot (Variables|Default|GetSaveGameRef) (Variables|Default|GetSaveGameSlot))
      (Default|CallGameSaved (Variables|Default|GetSaveGameRef)))))

(event Custom|CreateSaveGame
  (bind _returnvalue (SaveGame|CreateSaveGameObject "/Game/Blueprints/BP_SaveGame.BP_SaveGame_C"))
  (Variables|Default|SetSaveGameRef _returnvalue))

(event Custom|LoadGame
  (params (Async :type Boolean))
  (bind _savegameslot (Variables|Default|GetSaveGameSlot))
  (bind _returnvalue (SaveGame|DoesSaveGameExist (Variables|Default|GetSaveGameSlot)))
  (if _returnvalue
    (if Async
      (bind _savegame (|AsyncLoadGamefromSlot _savegameslot)
        (:Completed
          (bind _asbp_save_game (Utilities|Casting|CastToBP_SaveGame _savegame))
          (bind _output_get (Variables|Default|SetSaveGameRef _asbp_save_game))
          (Default|CallGameLoaded _output_get)))
      (else
        (bind _returnvalue_2 (SaveGame|LoadGamefromSlot _savegameslot))
        (bind _asbp_save_game_2 (Utilities|Casting|CastToBP_SaveGame _returnvalue_2))
        (bind _output_get_2 (Variables|Default|SetSaveGameRef _asbp_save_game_2))
        (Default|CallGameLoaded _output_get_2)))))

(event EventRequestSave
  (params (Async :type Boolean))
  (bind _outactors (Actor|GetAllActorswithInterface "/Game/Blueprints/BPI_Saveable.BPI_Saveable_C"))
  (Default|SaveAllData (Variables|Default|GetSaveGameRef) _outactors)
  (CallFunction|SaveGame Async))

(event EventRequestLoad
  (params (Requester :type Object%20Object%20Reference))
  (Default|LoadDataforRequester (Variables|Default|GetSaveGameRef) Requester))