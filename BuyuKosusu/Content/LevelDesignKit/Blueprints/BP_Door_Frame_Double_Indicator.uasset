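; Level design kit double door frame that color-codes the importance of the path through it.
; The Construction Script checks the importance enum and sets the frame mesh's first material slot to yellow for Golden Path, green for Side Path or red for Locked.
; Any other value resets the enum to its Golden default without applying a material in that pass.
; Event Graph holds no active logic.
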(event EventBeginPlay)

(event Collision|EventActorBeginOverlap
  (params (OtherActor :type Actor%20Object%20Reference)))

(event EventTick
  (params (DeltaSeconds :type Float%20%28single-precision%29)))

(fn ConstructionScript
  ;[1 1 1] Check if Importance level = Golden Path
  (if (== (Variables|Default|GetGoldenPath) (Variables|ImportanceLevel|GetEnum_ImportanceLevel))
    ;[1 1 1] Equals - Golden Path
    (Rendering|Material|SetMaterial (Variables|Default|GetSM_DoubleDoorFrame) 0 "/Game/LevelDesignKit/Material/MI_Color_Yellow.MI_Color_Yellow")
    (else
      ;[1 1 1] Check if Importance = Side Path
      (if (== (Variables|Default|GetSidePath) (Variables|ImportanceLevel|GetEnum_ImportanceLevel))
        (Rendering|Material|SetMaterial (Variables|Default|GetSM_DoubleDoorFrame) 0 "/Game/LevelDesignKit/Material/MI_Color_Green.MI_Color_Green")
        (else
          ;[1 1 1] Check if Importance = Locked
          (if (== (Variables|Default|GetLockedPath) (Variables|ImportanceLevel|GetEnum_ImportanceLevel))
            (Rendering|Material|SetMaterial (Variables|Default|GetSM_DoubleDoorFrame) 0 "/Game/LevelDesignKit/Material/MI_Color_Red.MI_Color_Red")
            (else
              ;[1 1 1] Rest to Golden
              (Variables|ImportanceLevel|SetEnum_ImportanceLevel "NewEnumerator0"))))))))