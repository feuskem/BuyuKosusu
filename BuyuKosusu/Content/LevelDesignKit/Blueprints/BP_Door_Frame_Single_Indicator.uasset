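; BP_Door_Frame_Single_Indicator is a level design kit door frame that color-codes the importance of its path.
; The construction script reads the importance enum and sets the main frame mesh's first material to yellow for Golden Path, green for Side Path or red for Locked.
; Any other value resets the enum to its first entry, commented as Golden, without applying a material in that pass.
; The event graph has no active logic.
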(event EventBeginPlay)

(event Collision|EventActorBeginOverlap
  (params (OtherActor :type Actor%20Object%20Reference)))

(event EventTick
  (params (DeltaSeconds :type Float%20%28single-precision%29)))

(fn ConstructionScript
  ;[1 1 1] Check Importance Level
  (if (== (Variables|Default|GetGoldenPath) (Variables|ImportanceLevel|GetEnumb_ImportanceLevel))
    ;[1 1 1] Importance = Golden Path
    (Rendering|Material|SetMaterial (Variables|Default|GetSM_MainDoorFrame) 0 "/Game/LevelDesignKit/Material/MI_Color_Yellow.MI_Color_Yellow")
    (else
      ;[1 1 1] Check if Importance = Side Path
      (if (== (Variables|Default|GetSidePath) (Variables|ImportanceLevel|GetEnumb_ImportanceLevel))
        (Rendering|Material|SetMaterial (Variables|Default|GetSM_MainDoorFrame) 0 "/Game/LevelDesignKit/Material/MI_Color_Green.MI_Color_Green")
        (else
          ;[1 1 1] Check if Importance = Locked
          (if (== (Variables|Default|GetLockedPath) (Variables|ImportanceLevel|GetEnumb_ImportanceLevel))
            (Rendering|Material|SetMaterial (Variables|Default|GetSM_MainDoorFrame) 0 "/Game/LevelDesignKit/Material/MI_Color_Red.MI_Color_Red")
            (else
              ;[1 1 1] Reset Value to Golden
              (Variables|ImportanceLevel|SetEnumb_ImportanceLevel "NewEnumerator0"))))))))