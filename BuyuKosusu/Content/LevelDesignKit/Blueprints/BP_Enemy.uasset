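; BP_Enemy is a level design kit enemy that dies as soon as something overlaps its damage radius or its Hit event fires.
; Death tips the rifle-pose mesh over with a timeline and sets the death text, then after a delay disables collision and toggles off the body.
; BeginPlay initializes the text and prints Life and Damage, but the damage, pain text and grunt branch is disconnected, so health never affects death.
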(event OnComponentBeginOverlap(TV_Damage_Radius)
  (params (OverlappedComponent :type Primitive%20Component%20Object%20Reference) (OtherActor :type Actor%20Object%20Reference) (OtherComp :type Primitive%20Component%20Object%20Reference) (OtherBodyIndex :type Integer) (bFromSweep :type Boolean) (SweepResult :type Hit%20Result%20Structure%20%28by%20ref%29))
  ;[1 1 1] Check if Hit or Close
  ;[1 1 1] Trigger Death Sequence
  (|DeathSequence)
  (Variables|Default|SetEnemy%20Dead true)
  (Utilities|FlowControl|Delay 2.0)
  (|HideText_3)
  (|TurnOffCollision)
  (|NoMoreEnemy))

(event EventBeginPlay
  ;[1 1 1] Start - Setting Variables
  (|HideText)
  (|SetLifeValue)
  (|SetDamageValue))

(event Collision|EventHit
  (params (MyComp :type Primitive%20Component%20Object%20Reference) (Other :type Actor%20Object%20Reference) (OtherComp :type Primitive%20Component%20Object%20Reference) (bSelfMoved :type Boolean) (HitLocation :type Vector :default "0, 0, 0") (HitNormal :type Vector :default "0, 0, 0") (NormalImpulse :type Vector :default "0, 0, 0") (Hit :type Hit%20Result%20Structure%20%28by%20ref%29))
  ;[1 1 1] Check if Hit or Close
  ;[1 1 1] Trigger Death Sequence
  (|DeathSequence)
  (Variables|Default|SetEnemy%20Dead true)
  (Utilities|FlowControl|Delay 2.0)
  (|HideText_3)
  (|TurnOffCollision)
  (|NoMoreEnemy))

(fn ConstructionScript)