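; Interactable button Blueprint that the player toggles on and off with the E key.
; Overlapping the TV_Press trigger volume enables input from player controller 0, and leaving it disables input, without checking which actor overlapped.
; Each press runs a FlipFlop that swaps the button mesh between green and red materials and plays the matching on or off 2D sound.
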(event OnComponentBeginOverlap(TV_Press)
  (params (OverlappedComponent :type Primitive%20Component%20Object%20Reference) (OtherActor :type Actor%20Object%20Reference) (OtherComp :type Primitive%20Component%20Object%20Reference) (OtherBodyIndex :type Integer) (bFromSweep :type Boolean) (SweepResult :type Hit%20Result%20Structure%20%28by%20ref%29))
  ;[1 1 1] Check If Player is CLose to Button
  (Input|EnableInput (Game|GetPlayerController 0)))

(event OnComponentEndOverlap(TV_Press)
  (params (OverlappedComponent :type Primitive%20Component%20Object%20Reference) (OtherActor :type Actor%20Object%20Reference) (OtherComp :type Primitive%20Component%20Object%20Reference) (OtherBodyIndex :type Integer))
  ;[1 1 1] Check If Player is CLose to Button
  (Input|DisableInput (Game|GetPlayerController 0)))

(event Input|KeyboardEvents|E
  (params (Key :type Key%20Structure))
  ;[1 1 1] Press E - Change Button Colour
  (:Pressed
    (Utilities|FlowControl|FlipFlop
      (:A
        (Rendering|Material|SetMaterial (Variables|Default|GetSM_Button) 0 "/Game/LevelDesignKit/Material/MI_Color_Green.MI_Color_Green")
        (Audio|PlaySound2D "/Game/LevelDesignKit/Audio/SFX_ButtonPressed_On.SFX_ButtonPressed_On" 1.0 1.0 0.0 0 0))
      (:B
        (Rendering|Material|SetMaterial (Variables|Default|GetSM_Button) 0 "/Game/LevelDesignKit/Material/MI_Color_Red.MI_Color_Red")
        (Audio|PlaySound2D "/Game/LevelDesignKit/Audio/SFX_ButtonPressed_Off.SFX_ButtonPressed_Off" 1.0 1.0 0.0 0 0)))))

(fn ConstructionScript)