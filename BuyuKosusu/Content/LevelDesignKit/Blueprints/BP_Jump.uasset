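; BP_Jump is a level design kit jumping-gap piece with low and high variants, selected by the HighJump flag.
; The construction script hides the meshes and markers of the unused variant.
; Trigger volume overlaps check the flag and teleport player 0 to the left or right destination component.
; The right trigger only handles the low jump, as the high-right teleport is never called.
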(event OnComponentBeginOverlap(TV_JumpRight)
  (params (OverlappedComponent :type Primitive%20Component%20Object%20Reference) (OtherActor :type Actor%20Object%20Reference) (OtherComp :type Primitive%20Component%20Object%20Reference) (OtherBodyIndex :type Integer) (bFromSweep :type Boolean) (SweepResult :type Hit%20Result%20Structure%20%28by%20ref%29))
  ;[1 1 1] Check Which Jump is Active to then teleport player to correct 'Right'
  (if (not (Variables|JumpHeight|GetHighJump))
    (|TeleportPlayerRightLow)))

(event OnComponentBeginOverlap(TV_LeftHigh)
  (params (OverlappedComponent :type Primitive%20Component%20Object%20Reference) (OtherActor :type Actor%20Object%20Reference) (OtherComp :type Primitive%20Component%20Object%20Reference) (OtherBodyIndex :type Integer) (bFromSweep :type Boolean) (SweepResult :type Hit%20Result%20Structure%20%28by%20ref%29))
  ;[1 1 1] If Active Send Players to the left
  (if (Variables|JumpHeight|GetHighJump)
    (|TeleportPlayerLeft_2)))

(event OnComponentBeginOverlap(TV_LeftLow)
  (params (OverlappedComponent :type Primitive%20Component%20Object%20Reference) (OtherActor :type Actor%20Object%20Reference) (OtherComp :type Primitive%20Component%20Object%20Reference) (OtherBodyIndex :type Integer) (bFromSweep :type Boolean) (SweepResult :type Hit%20Result%20Structure%20%28by%20ref%29))
  ;[1 1 1] If Active Send Players to the left
  (if (not (Variables|JumpHeight|GetHighJump))
    (|TeleportPlayerLeft)))

(fn ConstructionScript
  (if (Variables|JumpHeight|GetHighJump)
    (|HideLowJump)
    (else
      (|HideHighJump))))