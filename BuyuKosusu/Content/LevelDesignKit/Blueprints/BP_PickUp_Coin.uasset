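; BP_PickUp_Coin is a level design kit coin pickup that spins around its yaw axis each Tick until collected.
; An overlap on the pickup trigger volume hides the icon mesh, disables collision, prints a message, plays a 2D sound and sets the Collected flag.
; The overlap does not filter the overlapping actor, and the coin is neither destroyed nor added to any counter.
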(event OnComponentBeginOverlap(TV_PickUp)
  (params (OverlappedComponent :type Primitive%20Component%20Object%20Reference) (OtherActor :type Actor%20Object%20Reference) (OtherComp :type Primitive%20Component%20Object%20Reference) (OtherBodyIndex :type Integer) (bFromSweep :type Boolean) (SweepResult :type Hit%20Result%20Structure%20%28by%20ref%29))
  ;[1 1 1] Pick Up Object
  (if (not (Variables|Default|GetCollected))
    (|CoinDsappears)
    (Development|PrintString "You Picked up 1 Coin")
    (Variables|Default|SetCollected true)
    (Audio|PlaySound2D "/Game/LevelDesignKit/Audio/SFX_PickUp.SFX_PickUp" 1.0 1.0 0.0 0 0)))

(event EventTick
  (params (DeltaSeconds :type Float%20%28single-precision%29))
  ;[1 1 1] Make Object Spin
  (if (not (Variables|Default|GetCollected))
    (Transformation|AddLocalRotation (Variables|Default|GetSM_CoinPickUpIcon) (Math|Rotator|MakeRotator 0.0 0.0 (* DeltaSeconds (Variables|Default|GetRotation))) false false)))

(fn ConstructionScript)