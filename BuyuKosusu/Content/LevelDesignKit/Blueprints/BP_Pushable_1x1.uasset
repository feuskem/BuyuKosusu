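; BP_Pushable_1x1 is a level design kit block that shifts one step when one of its four side triggers is overlapped.
; Each push trigger's begin-overlap event adds a world offset to the block mesh, with no check on what overlapped it.
; Right and Left move it along world Y, North and South along X.
; Both axes share two distance variables: MoveDistanceRight for Right and North, MoveDistanceLeft for Left and South.
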(event OnComponentBeginOverlap(TV_Push_Right)
  (params (OverlappedComponent :type Primitive%20Component%20Object%20Reference) (OtherActor :type Actor%20Object%20Reference) (OtherComp :type Primitive%20Component%20Object%20Reference) (OtherBodyIndex :type Integer) (bFromSweep :type Boolean) (SweepResult :type Hit%20Result%20Structure%20%28by%20ref%29))
  (Transformation|AddWorldOffset (Variables|Default|GetSM_PushableObject_1x1x2) (Math|Vector|MakeVector 0.0 (Variables|Default|GetMove_Distance_Right) 0.0) false false))

(event OnComponentBeginOverlap(TV_Push_Left)
  (params (OverlappedComponent :type Primitive%20Component%20Object%20Reference) (OtherActor :type Actor%20Object%20Reference) (OtherComp :type Primitive%20Component%20Object%20Reference) (OtherBodyIndex :type Integer) (bFromSweep :type Boolean) (SweepResult :type Hit%20Result%20Structure%20%28by%20ref%29))
  (Transformation|AddWorldOffset (Variables|Default|GetSM_PushableObject_1x1x2) (Math|Vector|MakeVector 0.0 (Variables|Default|GetMove_Distance_Left) 0.0) false false))

(event OnComponentBeginOverlap(TV_Push_South)
  (params (OverlappedComponent :type Primitive%20Component%20Object%20Reference) (OtherActor :type Actor%20Object%20Reference) (OtherComp :type Primitive%20Component%20Object%20Reference) (OtherBodyIndex :type Integer) (bFromSweep :type Boolean) (SweepResult :type Hit%20Result%20Structure%20%28by%20ref%29))
  (Transformation|AddWorldOffset (Variables|Default|GetSM_PushableObject_1x1x2) (Math|Vector|MakeVector (Variables|Default|GetMove_Distance_Left) 0.0 0.0) false false))

(event OnComponentBeginOverlap(TV_Push_North)
  (params (OverlappedComponent :type Primitive%20Component%20Object%20Reference) (OtherActor :type Actor%20Object%20Reference) (OtherComp :type Primitive%20Component%20Object%20Reference) (OtherBodyIndex :type Integer) (bFromSweep :type Boolean) (SweepResult :type Hit%20Result%20Structure%20%28by%20ref%29))
  (Transformation|AddWorldOffset (Variables|Default|GetSM_PushableObject_1x1x2) (Math|Vector|MakeVector (Variables|Default|GetMove_Distance_Right) 0.0 0.0) false false))

(fn ConstructionScript)