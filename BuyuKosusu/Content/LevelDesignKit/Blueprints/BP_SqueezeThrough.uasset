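; BP_SqueezeThrough is a level design kit squeeze-through obstacle with 1m and 3m variants, chosen by the LongSqueeze flag.
; The construction script hides and disables collision on the unused variant's mesh and trigger, and BeginPlay enables collision for the selected one.
; Overlapping either trigger slows global time dilation to simulate squeezing, with no actor filter, and leaving restores normal speed.
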(event OnComponentBeginOverlap(TV_LongSqueezeThrough)
  (params (OverlappedComponent :type Primitive%20Component%20Object%20Reference) (OtherActor :type Actor%20Object%20Reference) (OtherComp :type Primitive%20Component%20Object%20Reference) (OtherBodyIndex :type Integer) (bFromSweep :type Boolean) (SweepResult :type Hit%20Result%20Structure%20%28by%20ref%29))
  ;[1 1 1] 3m SqueezeThrough
  (Utilities|Time|SetGlobalTimeDilation 0.35))

(event OnComponentBeginOverlap(TV_ShortSqueezeThrough)
  (params (OverlappedComponent :type Primitive%20Component%20Object%20Reference) (OtherActor :type Actor%20Object%20Reference) (OtherComp :type Primitive%20Component%20Object%20Reference) (OtherBodyIndex :type Integer) (bFromSweep :type Boolean) (SweepResult :type Hit%20Result%20Structure%20%28by%20ref%29))
  ;[1 1 1] 1m SqueezeThrough
  (Utilities|Time|SetGlobalTimeDilation 0.35))

(event OnComponentEndOverlap(TV_LongSqueezeThrough)
  (params (OverlappedComponent :type Primitive%20Component%20Object%20Reference) (OtherActor :type Actor%20Object%20Reference) (OtherComp :type Primitive%20Component%20Object%20Reference) (OtherBodyIndex :type Integer))
  ;[1 1 1] 3m SqueezeThrough
  (Utilities|Time|SetGlobalTimeDilation 1.0))

(event OnComponentEndOverlap(TV_ShortSqueezeThrough)
  (params (OverlappedComponent :type Primitive%20Component%20Object%20Reference) (OtherActor :type Actor%20Object%20Reference) (OtherComp :type Primitive%20Component%20Object%20Reference) (OtherBodyIndex :type Integer))
  ;[1 1 1] 1m SqueezeThrough
  (Utilities|Time|SetGlobalTimeDilation 1.0))

(event EventBeginPlay
  ;[1 1 1] Set Correct SqueezeThrough
  (if (Variables|SqueezeThrough|Length|GetLong%20Squeeze)
    (|LongSqueeze_Collision_Enabled)
    (else
      (|ShortSqueezeCollisionEnabled))))

(fn ConstructionScript
  ;[1 1 1] Setting Up Ladder Variation
  (if (Variables|SqueezeThrough|Length|GetLong%20Squeeze)
    (|HideShortSqueeze)
    (else
      (|HideLongSqueeze))))