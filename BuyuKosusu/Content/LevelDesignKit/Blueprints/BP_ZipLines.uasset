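; BP_ZipLines is a level-design zipline that moves the player by instant teleport rather than an animated slide.
; The Short flag makes the construction script toggle visibility on the unused 5m or 10m mesh and its destination marker.
; Any overlap on TV_Slide_Down teleports player character 0 to the location and rotation of TPShort or TPLong, according to that same flag.
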(event OnComponentBeginOverlap(TV_Slide_Down)
  (params (OverlappedComponent :type Primitive%20Component%20Object%20Reference) (OtherActor :type Actor%20Object%20Reference) (OtherComp :type Primitive%20Component%20Object%20Reference) (OtherBodyIndex :type Integer) (bFromSweep :type Boolean) (SweepResult :type Hit%20Result%20Structure%20%28by%20ref%29))
  (if (Variables|ZipLineLength|GetShort)
    (|TeleportPlayersShortZipline)
    (else
      (|TeleportPlayerstotheLeft_2))))

(fn ConstructionScript
  (if (Variables|ZipLineLength|GetShort)
    (Rendering|ToggleVisibility (Variables|Default|GetSM_ZipLines_10m) false)
    (Rendering|ToggleVisibility (Variables|Default|GetTP_Long) false)
    (else
      (Rendering|ToggleVisibility (Variables|Default|GetSM_ZipLines_5m) false)
      (Rendering|ToggleVisibility (Variables|Default|GetTP_Short) false))))