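; Level-design-kit lift that raises and lowers a floor platform, sized by name at 3m with a 4m height.
; Overlapping the in-lift trigger enables input for player 0; leaving disables it and hides both direction arrows, which also start hidden.
; Pressing E alternates through a FlipFlop between playing and reversing the LiftTravel timeline, which sets the floor's relative location, while showing the matching up or down arrow.
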(event OnComponentBeginOverlap(TV_InLift)
  (params (OverlappedComponent :type Primitive%20Component%20Object%20Reference) (OtherActor :type Actor%20Object%20Reference) (OtherComp :type Primitive%20Component%20Object%20Reference) (OtherBodyIndex :type Integer) (bFromSweep :type Boolean) (SweepResult :type Hit%20Result%20Structure%20%28by%20ref%29))
  ;[1 1 1] When InLift Allow Interaction
  (Input|EnableInput (Game|GetPlayerController 0)))

(event OnComponentEndOverlap(TV_InLift)
  (params (OverlappedComponent :type Primitive%20Component%20Object%20Reference) (OtherActor :type Actor%20Object%20Reference) (OtherComp :type Primitive%20Component%20Object%20Reference) (OtherBodyIndex :type Integer))
  ;[1 1 1] When InLift Allow Interaction
  (Input|DisableInput (Game|GetPlayerController 0))
  (|HideArrows_2))

(event EventBeginPlay
  ;[1 1 1] Hide Arrows
  (|HideArrows))

(event Input|KeyboardEvents|E
  (params (Key :type Key%20Structure :default "None"))
  ;[1 1 1] Move Lift on Key Press
  (:Pressed
    (Utilities|FlowControl|FlipFlop
      (:A
        (|Arrow_Visability
          (:Play
            (bind _newtrack_1 (Timeline|LiftTravel Play)
              (:Update
                (Transformation|SetRelativeLocation (Variables|Default|GetFloor4x4m) _newtrack_1 false false))))))
      (:B
        (|Arrow_Visability_2
          (:Play
            (Timeline|LiftTravel Reverse)))))))

(fn ConstructionScript)