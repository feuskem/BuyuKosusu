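; BP_CollapsingTunnel is a level mechanic that collapses a tunnel when an actor enters its TV_Collapse trigger volume.
; The overlap starts two timelines: RockFall moves SMRock02 along a track, and a second one pitches SMRock03 over, while SMRock01 snaps straight to a tilted rotation.
; A Collapsed flag, set during RockFall updates, blocks later overlaps from replaying the collapse.
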(event OnComponentBeginOverlap(TV_Collapse)
  (params (OverlappedComponent :type Primitive%20Component%20Object%20Reference) (OtherActor :type Actor%20Object%20Reference) (OtherComp :type Primitive%20Component%20Object%20Reference) (OtherBodyIndex :type Integer) (bFromSweep :type Boolean) (SweepResult :type Hit%20Result%20Structure%20%28by%20ref%29))
  ;[1 1 1] Enter Trigger Tunnel Collapses
  (if (not (Variables|Default|GetCollapsed))
    (Utilities|FlowControl|Sequence
      (:then_0
        (bind _newtrack_1 (Timeline|RockFall Play)
          (:Update
            (Transformation|SetRelativeLocation (Variables|Default|GetSM_Rock02) _newtrack_1 false false)
            (Variables|Default|SetCollapsed true))))
      (:then_1
        (bind _doorfloat (Timeline|Timeline Play)
          (:Update
            (Transformation|SetRelativeRotation (Variables|Default|GetSM_Rock03) (Math|Rotator|MakeRotator 0.0 (Math|Float|Lerp 0.0 6e+01 _doorfloat) 0.0) false false))))
      (:then_2
        (Transformation|SetRelativeRotation (Variables|Default|GetSM_Rock01) (Math|Rotator|MakeRotator 0.0 -35.0 0.0) false false)))))

(fn ConstructionScript)