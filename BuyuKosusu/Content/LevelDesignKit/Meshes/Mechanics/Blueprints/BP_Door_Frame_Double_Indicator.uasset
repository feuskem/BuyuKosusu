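; Level design kit double door frame that color-codes the importance of the path through it.
; The Construction Script compares ImportanceLevel to Golden, Side and Locked Path, then sets the frame mesh's first material to yellow, green or red respectively.
; Any other value resets ImportanceLevel to Golden Path without setting a material in that branch.
; The event graph holds only disabled stub events, so it adds no runtime logic.
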(event EventBeginPlay)

(event Collision|EventActorBeginOverlap
  (params (OtherActor :type Actor%20Object%20Reference)))

(event EventTick
  (params (DeltaSeconds :type Float%20%28single-precision%29)))

(fn ConstructionScript
  ;[1 1 1] Check if Importance level = Golden Path
  (if (== (Variables|Default|GetGoldenPath) (Variables|Default|GetImportanceLevel))
    ;[1 1 1] Equals - Golden Path
    (Rendering|Material|SetMaterial (Variables|Default|GetSM_DoubleDoorFrame) 0 "/Game/LevelDesignKit/Material/MI_Color_Yellow.MI_Color_Yellow")
    (else
      ;[1 1 1] Check if Importance = Side Path
      (if (== (Variables|Default|GetSidePath) (Variables|Default|GetImportanceLevel))
        (Rendering|Material|SetMaterial (Variables|Default|GetSM_DoubleDoorFrame) 0 "/Game/LevelDesignKit/Material/MI_Color_Green.MI_Color_Green")
        (else
          ;[1 1 1] Check if Importance = Locked
          (if (== (Variables|Default|GetLockedPath) (Variables|Default|GetImportanceLevel))
            (Rendering|Material|SetMaterial (Variables|Default|GetSM_DoubleDoorFrame) 0 "/Game/LevelDesignKit/Material/MI_Color_Red.MI_Color_Red")
            (else
              ;[1 1 1] Rest to Golden
              (Variables|Default|SetImportanceLevel (Variables|Default|GetGoldenPath)))))))))