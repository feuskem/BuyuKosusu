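; Lever-operated drawbridge that the player lowers once by pressing E inside the TV_PullLevar overlap volume.
; The construction script uses LongBridge to pick the standard or 10m mesh, hiding the other and disabling its collision.
; Overlap toggles actor input; E snaps the lever, enables bridge collision and plays that mesh's timeline to rotate it from raised to flat, setting BridgeDown to block repeats.
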(event OnComponentBeginOverlap(TV_PullLevar)
  (params (OverlappedComponent :type Primitive%20Component%20Object%20Reference) (OtherActor :type Actor%20Object%20Reference) (OtherComp :type Primitive%20Component%20Object%20Reference) (OtherBodyIndex :type Integer) (bFromSweep :type Boolean) (SweepResult :type Hit%20Result%20Structure%20%28by%20ref%29))
  ;[1 1 1] Check If pLayer is close to Levar#
  (Input|EnableInput (Game|GetPlayerController 0)))

(event OnComponentEndOverlap(TV_PullLevar)
  (params (OverlappedComponent :type Primitive%20Component%20Object%20Reference) (OtherActor :type Actor%20Object%20Reference) (OtherComp :type Primitive%20Component%20Object%20Reference) (OtherBodyIndex :type Integer))
  ;[1 1 1] Check If pLayer is close to Levar#
  (Input|DisableInput (Game|GetPlayerController 0)))

(event Input|KeyboardEvents|E
  (params (Key :type Key%20Structure :default "None"))
  (:Pressed
    (if (not (Variables|Default|GetBridgeDown))
      ;[1 1 1] Rotate Levar
      (Transformation|SetRelativeRotation (Variables|Default|GetSM_LeverLarge) (Math|Rotator|MakeRotator 0.0 0.0 0.0) false false)
      (if (Variables|Bridge|Length|GetLongBridge)
        ;[1 1 1] Rotate Bridge_Long Bridge
        (Collision|SetCollisionEnabled (Variables|Default|GetST_BridgeStraight10m) "QueryAndPhysics")
        (bind _newtrack_0 (Timeline|Timeline Play)
          (:Update
            (Transformation|SetRelativeRotation (Variables|Default|GetST_BridgeStraight10m) (Math|Rotator|MakeRotator (Math|Float|Lerp 9e+01 0.0 _newtrack_0) 0.0 9e+01) false false)))
        (else
          ;[1 1 1] Rotate Bridge
          (Collision|SetCollisionEnabled (Variables|Default|GetST_BridgeStraight) "QueryAndPhysics")
          (bind _newtrack_0_2 (Timeline|BridgeComesDown Play)
            (:Update
              (Transformation|SetRelativeRotation (Variables|Default|GetST_BridgeStraight) (Math|Rotator|MakeRotator (Math|Float|Lerp 9e+01 0.0 _newtrack_0_2) 0.0 9e+01) false false)))))
      ;[1 1 1] Bridge Complete
      (Variables|Default|SetBridgeDown true))))

(fn ConstructionScript
  (bind _st_bridgestraight10m (Variables|Default|GetST_BridgeStraight10m))
  (if (Variables|Bridge|Length|GetLongBridge)
    (Rendering|SetVisibility (Variables|Default|GetST_BridgeStraight) false false)
    (Collision|SetCollisionEnabled (Variables|Default|GetST_BridgeStraight) "NoCollision")
    (else
      (Rendering|SetVisibility _st_bridgestraight10m false false)
      (Collision|SetCollisionEnabled _st_bridgestraight10m "NoCollision"))))