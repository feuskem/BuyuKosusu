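; BP_Lock_and_Key is a level-design-kit mechanic pairing a collectible key with a lock that opens once the key is held.
; Overlapping the key trigger sets HasKey and hides the key icon.
; Overlapping the lock trigger with the key swaps the closed lock icon for the open one, hidden at BeginPlay, and sets LockOpen so it happens once.
; Neither trigger filters the overlapping actor.
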(event OnComponentBeginOverlap(TV_CloseToLock)
  (params (OverlappedComponent :type Primitive%20Component%20Object%20Reference) (OtherActor :type Actor%20Object%20Reference) (OtherComp :type Primitive%20Component%20Object%20Reference) (OtherBodyIndex :type Integer) (bFromSweep :type Boolean) (SweepResult :type Hit%20Result%20Structure%20%28by%20ref%29))
  ;[1 1 1] Opening Lock
  (if (not (Variables|Default|GetLockOpen))
    (if (Variables|Default|GetHasKey)
      (Rendering|SetVisibility (Variables|Default|GetSM_LockIcon_Open) true false)
      (Rendering|SetVisibility (Variables|Default|GetSM_LockIcon) false false)
      (Variables|Default|SetLockOpen true))))

(event OnComponentBeginOverlap(TV_Key)
  (params (OverlappedComponent :type Primitive%20Component%20Object%20Reference) (OtherActor :type Actor%20Object%20Reference) (OtherComp :type Primitive%20Component%20Object%20Reference) (OtherBodyIndex :type Integer) (bFromSweep :type Boolean) (SweepResult :type Hit%20Result%20Structure%20%28by%20ref%29))
  ;[1 1 1] Player PicksUp Key
  (Variables|Default|SetHasKey true)
  (Rendering|SetVisibility (Variables|Default|GetSM_KeyIcon) false false))

(event EventBeginPlay
  ;[1 1 1] Hide Lock Open
  (Rendering|SetVisibility (Variables|Default|GetSM_LockIcon_Open) false false))

(fn ConstructionScript)