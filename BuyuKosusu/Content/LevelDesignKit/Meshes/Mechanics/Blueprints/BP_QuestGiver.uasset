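; BP_QuestGiver is a level design kit quest-giver marker that shows an exclamation point icon and a sticky note of quest text.
; The construction script fills the header and three text lines from variables.
; BeginPlay toggles the note and its child components to start hidden.
; Entering or leaving the TV_Approach_NPC trigger flips note and icon visibility, without filtering the overlapping actor or setting explicit states.
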(event OnComponentBeginOverlap(TV_Approach_NPC)
  (params (OverlappedComponent :type Primitive%20Component%20Object%20Reference) (OtherActor :type Actor%20Object%20Reference) (OtherComp :type Primitive%20Component%20Object%20Reference) (OtherBodyIndex :type Integer) (bFromSweep :type Boolean) (SweepResult :type Hit%20Result%20Structure%20%28by%20ref%29))
  ;[1 1 1] Show Quest Text
  (Rendering|ToggleVisibility (Variables|Default|GetSM_StickyNote) true)
  (Rendering|ToggleVisibility (Variables|Default|GetSM_ExclamationPoint) false))

(event OnComponentEndOverlap(TV_Approach_NPC)
  (params (OverlappedComponent :type Primitive%20Component%20Object%20Reference) (OtherActor :type Actor%20Object%20Reference) (OtherComp :type Primitive%20Component%20Object%20Reference) (OtherBodyIndex :type Integer))
  ;[1 1 1] Show Quest Icon
  (Rendering|ToggleVisibility (Variables|Default|GetSM_StickyNote) true)
  (Rendering|ToggleVisibility (Variables|Default|GetSM_ExclamationPoint) false))

(event EventBeginPlay
  ;[1 1 1] Hide Text Box
  (Rendering|ToggleVisibility (Variables|Default|GetSM_StickyNote) true))

(fn ConstructionScript
  (Rendering|Components|TextRender|SetText (Variables|Default|GetTxt_QuestNumber) (Variables|QuestText|GetQuestHeader))
  (Rendering|Components|TextRender|SetText (Variables|Default|GetTxt_Line_01) (Variables|QuestText|GetQuest_Text_01))
  (Rendering|Components|TextRender|SetText (Variables|Default|GetTxt_Line_02) (Variables|QuestText|GetQuest_Text_02))
  (Rendering|Components|TextRender|SetText (Variables|Default|GetTxt_Line_03) (Variables|QuestText|GetQuest_Text_03)))