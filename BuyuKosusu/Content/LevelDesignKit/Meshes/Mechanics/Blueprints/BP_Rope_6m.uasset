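; BP_Rope_6m is a level design kit rope that moves the player between its two ends by teleporting.
; Overlap volumes at the top and bottom each trigger a function that teleports player character 0 to a marker component at the opposite end, taking that marker's location and rotation.
; The overlapping actor is never checked, so anything entering either volume teleports the player.
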(event OnComponentBeginOverlap(TV_Rop_Bottom)
  (params (OverlappedComponent :type Primitive%20Component%20Object%20Reference) (OtherActor :type Actor%20Object%20Reference) (OtherComp :type Primitive%20Component%20Object%20Reference) (OtherBodyIndex :type Integer) (bFromSweep :type Boolean) (SweepResult :type Hit%20Result%20Structure%20%28by%20ref%29))
  (|TeleportPlayeTotheTop))

(event OnComponentBeginOverlap(TV_Rop_Top)
  (params (OverlappedComponent :type Primitive%20Component%20Object%20Reference) (OtherActor :type Actor%20Object%20Reference) (OtherComp :type Primitive%20Component%20Object%20Reference) (OtherBodyIndex :type Integer) (bFromSweep :type Boolean) (SweepResult :type Hit%20Result%20Structure%20%28by%20ref%29))
  (|TeleportPlayeTotheBottom))

(fn ConstructionScript)