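; BP_SwingPole is a level design kit swing pole that moves the player to either side of it by teleporting, with no swing motion in its graphs.
; Overlapping the right or left trigger volume teleports player character 0 to the location and rotation of TPRight or TPLeft respectively, without checking the overlapping actor.
; The construction script uses the Short flag to toggle visibility on either the 3m or 2m pole mesh.
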(event OnComponentBeginOverlap(TV_Swing_Right)
  (params (OverlappedComponent :type Primitive%20Component%20Object%20Reference) (OtherActor :type Actor%20Object%20Reference) (OtherComp :type Primitive%20Component%20Object%20Reference) (OtherBodyIndex :type Integer) (bFromSweep :type Boolean) (SweepResult :type Hit%20Result%20Structure%20%28by%20ref%29))
  (|TeleportPlayerstotheRight_2))

(event OnComponentBeginOverlap(TV_Swing_Left)
  (params (OverlappedComponent :type Primitive%20Component%20Object%20Reference) (OtherActor :type Actor%20Object%20Reference) (OtherComp :type Primitive%20Component%20Object%20Reference) (OtherBodyIndex :type Integer) (bFromSweep :type Boolean) (SweepResult :type Hit%20Result%20Structure%20%28by%20ref%29))
  (|TeleportPlayerstotheLeft_2))

(fn ConstructionScript
  (if (Variables|PoleLength|GetShort)
    (Rendering|ToggleVisibility (Variables|Default|GetSM_SwingPole3m) false)
    (else
      (Rendering|ToggleVisibility (Variables|Default|GetSM_SwingPole2m) false))))