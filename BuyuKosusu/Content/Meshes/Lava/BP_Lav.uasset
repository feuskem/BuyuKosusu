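; BP_Lav is a lava volume that destroys fireballs and hampers the first-person character while it overlaps.
; Its ProjectileDestroyer415 component's begin overlap destroys any BP_Fireball, or caches the character and calls Slow.
; Slow re-arms itself on a short looping timer, repeatedly applying configured walk speed and jump velocity and setting the character's flag A.
; End overlap clears the timer and flag, then restores hardcoded movement values.
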(event OnComponentBeginOverlap(ProjectileDestroyer415)
  (params (OverlappedComponent :type Primitive%20Component%20Object%20Reference) (OtherActor :type Actor%20Object%20Reference) (OtherComp :type Primitive%20Component%20Object%20Reference) (OtherBodyIndex :type Integer) (bFromSweep :type Boolean) (SweepResult :type Hit%20Result%20Structure%20%28by%20ref%29))
  (Utilities|FlowControl|Sequence
    (:then_0
      (bind _asbp_fireball (Utilities|Casting|CastToBP_Fireball OtherActor))
      (Actor|DestroyActor _asbp_fireball))
    (:then_1
      (bind _asbp_first_person_character (Utilities|Casting|CastToBP_FirstPersonCharacter OtherActor))
      (Variables|Default|SetAs%20BP%20First%20Person%20Character _asbp_first_person_character)
      (CallFunction|Slow))))

(event OnComponentBeginOverlap(EnemyHealthUpdater)
  (params (OverlappedComponent :type Primitive%20Component%20Object%20Reference) (OtherActor :type Actor%20Object%20Reference) (OtherComp :type Primitive%20Component%20Object%20Reference) (OtherBodyIndex :type Integer) (bFromSweep :type Boolean) (SweepResult :type Hit%20Result%20Structure%20%28by%20ref%29)))

(event OnComponentBeginOverlap(PlayerBlock)
  (params (OverlappedComponent :type Primitive%20Component%20Object%20Reference) (OtherActor :type Actor%20Object%20Reference) (OtherComp :type Primitive%20Component%20Object%20Reference) (OtherBodyIndex :type Integer) (bFromSweep :type Boolean) (SweepResult :type Hit%20Result%20Structure%20%28by%20ref%29)))

(event OnComponentEndOverlap(ProjectileDestroyer415)
  (params (OverlappedComponent :type Primitive%20Component%20Object%20Reference) (OtherActor :type Actor%20Object%20Reference) (OtherComp :type Primitive%20Component%20Object%20Reference) (OtherBodyIndex :type Integer))
  (bind _asbp_first_person_character (Utilities|Casting|CastToBP_FirstPersonCharacter OtherActor))
  (Utilities|Time|ClearandInvalidateTimerbyHandle (stale Custom|Slow _returnvalue))
  (Variables|/Script/Engine.CharacterMovementComponent|SetMaxWalkSpeed (Variables|/Script/Engine.Character|GetCharacterMovement _asbp_first_person_character) 6e+02)
  (Variables|/Game/FirstPerson/Blueprints/BP_FirstPersonCharacter.BP_FirstPersonCharacter_C|SetA _asbp_first_person_character false)
  (Variables|/Script/Engine.CharacterMovementComponent|SetJumpZVelocity (Variables|/Script/Engine.Character|GetCharacterMovement (Variables|Default|GetAs%20BP%20First%20Person%20Character)) 6.5e+02))

(event Custom|Slow
  (bind _as_bp_first_person_character (Variables|Default|GetAs%20BP%20First%20Person%20Character))
  (bind _charactermovement (Variables|/Script/Engine.Character|GetCharacterMovement _as_bp_first_person_character))
  (bind _returnvalue (Utilities|Time|SetTimerbyEvent (delegate Custom|Slow) 0.1 true))
  (Variables|/Script/Engine.CharacterMovementComponent|SetMaxWalkSpeed _charactermovement (Variables|Default|GetMax%20Walk%20Speed))
  (Variables|/Game/FirstPerson/Blueprints/BP_FirstPersonCharacter.BP_FirstPersonCharacter_C|SetA _as_bp_first_person_character true)
  (Variables|/Script/Engine.CharacterMovementComponent|SetJumpZVelocity _charactermovement (Variables|Default|GetJump%20Z%20Velocity)))

(event EventBeginPlay)

(event Collision|EventActorBeginOverlap
  (params (OtherActor :type Actor%20Object%20Reference)))

(event EventTick
  (params (DeltaSeconds :type Float%20%28single-precision%29)))

(event Collision|EventActorEndOverlap
  (params (OtherActor :type Actor%20Object%20Reference)))

(fn ConstructionScript)