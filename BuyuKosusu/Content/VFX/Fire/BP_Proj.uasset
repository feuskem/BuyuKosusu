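; BP_Proj is a fire VFX projectile that launches itself on spawn and fades out on first impact.
; BeginPlay gives the physics Sphere a randomized forward velocity-change impulse.
; The first hit, gated by DoOnce, disables physics and collision and deactivates the Projectile effect.
; A Size timeline then drives the effect's "User Size" parameter and destroys the actor when finished.
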(event OnComponentHit(Sphere)
  (params (HitComponent :type Primitive%20Component%20Object%20Reference) (OtherActor :type Actor%20Object%20Reference) (OtherComp :type Primitive%20Component%20Object%20Reference) (NormalImpulse :type Vector :default "0, 0, 0") (Hit :type Hit%20Result%20Structure%20%28by%20ref%29))
  (bind _sphere (Variables|Default|GetSphere))
  (Utilities|FlowControl|DoOnce false
    (:Completed
      (Physics|SetSimulatePhysics _sphere false)
      (Collision|SetCollisionEnabled _sphere "NoCollision")
      (Components|Activation|Deactivate (Variables|Default|GetProjectile))
      (bind _size (Timeline|Size PlayFromStart)
        (:Update
          (Effects|Components|ParticleSystem|SetFloatParameter (Variables|Default|GetProjectile) "User Size" _size))
        (:Finished
          (Actor|DestroyActor))))))

(event EventBeginPlay
  (Physics|AddImpulse (Variables|Default|GetSphere) (* (Math|Vector|GetForwardVector (Variables|Default|GetSphere)) (Math|Random|RandomFloatinRange 7.5e+02 1.3e+03)) "None" true))

(fn ConstructionScript)